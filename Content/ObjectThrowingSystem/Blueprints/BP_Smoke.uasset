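; BP_Smoke is a smoke actor in the object throwing system that scales in, lingers for a set lifetime, then scales out and disappears.
; A timeline drives the fade-in scale on BeginPlay, while the authority waits out SmokeLifeTime and fires a multicast event.
; That multicast plays the fade-out scale timeline, and only the authority destroys the actor when it finishes.
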(event `self.ReceiveBeginPlay`
  (`|ExecutionSequence`
    (:`then_0`
      (bind (_direction _fade_in) (`Timeline|Animation Fade In` :!via `PlayFromStart`)
        (:`Update`
          (`self.SetActorScale3D` (`KismetMathLibrary.Conv_DoubleToVector` _fade_in)))))
    (:`then_1`
      (`/Engine/EditorBlueprintResources/ActorMacros.Switch Has Authority`
        (:`Authority`
          (`KismetSystemLibrary.Delay` (`self.Smoke Life Time`))
          (`self.MULTICAST Fire disappear`))))))

(event `MULTICAST Fire Disappear`
  ;[1 1 1] Play Animation
  (bind (_direction _animation) (`Timeline|Animation Fade Out` :!via `PlayFromStart`)
    (:`Update`
      (`self.SetActorRelativeScale3D` (`KismetMathLibrary.Conv_DoubleToVector` _animation)))
    (:`Finished`
      (`/Engine/EditorBlueprintResources/ActorMacros.Switch Has Authority`
        (:`Authority`
          (`self.K2_DestroyActor`))))))

(fn `UserConstructionScript`)