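; Destructible wave spawner that starts once the player character enters its trigger box and destroys itself when its HP runs out.
; After a placeholder start timeline, timers step through SpawnInfos, spawning each wave's actors across five spawn points with a sound and registering them with an optional DoorActor.
; An end timeline, also just printing debug text, plays after the last wave.
; Tick turns the health bar toward the player camera.
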(event `self.ReceiveActorBeginOverlap`
  (params (OtherActor :type "Actor Object Reference"))
  (`parent.ReceiveActorBeginOverlap` OtherActor))

(event `self.ReceiveBeginPlay`
  (`parent.ReceiveBeginPlay`)
  (set `self.SpwanLocations` (`|MakeArray` (`self.SpawnPoint`) (`self.SpawnPoint1`) (`self.SpawnPoint2`) (`self.SpawnPoint3`) (`self.SpawnPoint4`))))

(event `self.ReceiveTick`
  (params (DeltaSeconds :type "Float (single-precision)"))
  (`SceneComponent.K2_SetWorldRotation` (`self.NPC Blood Strip`) (`KismetMathLibrary.FindLookAtRotation` (`self.K2_GetActorLocation`) (`self.K2_GetActorLocation` (`PlayerController.PlayerCameraManager` (`GameplayStatics.GetPlayerController` 0)))) false false))

(event `self.Box.OnComponentBeginOverlap`
  (params (OverlappedComponent :type "PrimitiveComponent Object Reference") (OtherActor :type "Actor Object Reference") (OtherComp :type "PrimitiveComponent Object Reference") (OtherBodyIndex :type Integer) (bFromSweep :type Boolean) (SweepResult :type "HitResult Structure (by ref)"))
  (cast `/Game/CombatSystem/Blueprints/BP_CombatCharacter_Player` OtherActor)
  (`/Engine/EditorBlueprintResources/StandardMacros.DoOnce` false
    (:`Completed`
      (`Timeline|Start` :!via `PlayFromStart`
        (:`Update`
          (`KismetSystemLibrary.PrintString` "播放出现动画"))
        (:`Finished`
          (`self.StartWork`))))))

(event `StartWork`
  (if (>= (- (`KismetArrayLibrary.Array_Length` (`self.SpawnInfos`)) 1) (`self.CurrentSpawnIndex`))
    (`KismetSystemLibrary.K2_SetTimerDelegate` (delegate `SpawnNext`) (`.NeedWaitTime_5_00753E824714DC7518780A89885260EB` (break `/Game/AISpwaner/S_SpawnInfo` (`|GetArrayItem` (`self.SpawnInfos`) (`self.CurrentSpawnIndex`)))))
    (else
      (`/Engine/EditorBlueprintResources/StandardMacros.DoOnce` false :!label _label
        (:`Completed`
          (`Timeline|FinishSpawn` :!via `PlayFromStart`
            (:`Update`
              (`KismetSystemLibrary.PrintString` "播放结束动画"))))))))

(event `SpawnNext`
  (bind _door_actor (`self.Door Actor`))
  (bind (_spwanactor _needwaittime _number) (break `/Game/AISpwaner/S_SpawnInfo` (`|GetArrayItem` (`self.SpawnInfos`) (`self.CurrentSpawnIndex`))))
  (if (>= (- (`KismetArrayLibrary.Array_Length` (`self.SpawnInfos`)) 1) (`self.CurrentSpawnIndex`))
    (for _index (range _number)
      (bind _output (`|GetArrayItem` (`self.SpwanLocations`) _index))
      (bind _returnvalue (`SceneComponent.K2_GetComponentLocation` _output))
      (bind _returnvalue_2 (`|SpawnActorFromClass` _spwanactor (`KismetMathLibrary.MakeTransform` _returnvalue (`SceneComponent.K2_GetComponentRotation` _output)) "Undefined" "MultiplyWithRoot" null null))
      (`GameplayStatics.PlaySoundAtLocation` "/Game/CombatSystem/CourseFiles/SoundFX/A_Character_Heal01.A_Character_Heal01" _returnvalue (struct) 1.0 1.0 0.0 null null null null)
      (`/Engine/EditorBlueprintResources/StandardMacros.IsValid` _door_actor
        (:`Is Valid`
          (`/Game/CombatSystem/AI/BP_Door.动态添加NPC` _door_actor _returnvalue_2))))
    (set `self.CurrentSpawnIndex` (+ (`self.CurrentSpawnIndex`) 1))
    (`self.StartWork`)
    (else
      (goto _label))))

(event `self.C_NPC_Status_Component.Attack Feedback Notification`
  (params (Actor :type "Actor Object Reference"))
  (bind (_npc_basic_data_maxhp _npc_basic_data_currenthp) (break `/Game/CombatSystem/AI/NPC/NPC_BasicData` (`/Game/CombatSystem/AI/NPC/C_NPC_Status_Component.NPC Basic Data` (`self.C_NPC_Status_Component`))))
  (if (not (> _npc_basic_data_currenthp 0.0))
    (`self.K2_DestroyActor`)))

(fn `UserConstructionScript`
  (`SceneComponent.K2_SetRelativeTransform` (`self.Box`) (`self.New Transform`) false false))