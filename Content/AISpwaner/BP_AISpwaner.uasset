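; BP_AISpwaner is a wave spawner that starts once, when a BP_CombatCharacter_Player first enters its Box.
; After the Start timeline, it works through SpawnInfos, waiting each entry's delay before spawning its actors at up to five spawn points with a sound.
; Each spawn gets an AIMoveTo toward DoorPosition, though GoalActor is set to itself.
; After the last wave, the FinishSpawn timeline calls CallFinishAISpawn on every update.
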(event `self.ReceiveBeginPlay`
  (set `self.SpwanLocations` (`|MakeArray` (`self.SpawnPoint`) (`self.SpawnPoint1`) (`self.SpawnPoint2`) (`self.SpawnPoint3`) (`self.SpawnPoint4`))))

(event `self.Box.OnComponentBeginOverlap`
  (params (OverlappedComponent :type "PrimitiveComponent Object Reference") (OtherActor :type "Actor Object Reference") (OtherComp :type "PrimitiveComponent Object Reference") (OtherBodyIndex :type Integer) (bFromSweep :type Boolean) (SweepResult :type "HitResult Structure (by ref)"))
  (cast `/Game/CombatSystem/Blueprints/BP_CombatCharacter_Player` OtherActor)
  (`/Engine/EditorBlueprintResources/StandardMacros.DoOnce` false
    (:`Completed`
      (`Timeline|Start` :!via `PlayFromStart`
        (:`Update`
          (`KismetSystemLibrary.PrintString` "播放出现动画"))
        (:`Finished`
          (`self.StartWork`))))))

(event `StartWork`
  (if (>= (- (`KismetArrayLibrary.Array_Length` (`self.SpawnInfos`)) 1) (`self.CurrentSpawnIndex`))
    (`KismetSystemLibrary.K2_SetTimerDelegate` (delegate `SpawnNext`) (`.NeedWaitTime_5_00753E824714DC7518780A89885260EB` (break `/Game/AISpwaner/S_SpawnInfo` (`|GetArrayItem` (`self.SpawnInfos`) (`self.CurrentSpawnIndex`)))))
    (else
      (`/Engine/EditorBlueprintResources/StandardMacros.DoOnce` false :!label _label
        (:`Completed`
          (`Timeline|FinishSpawn` :!via `PlayFromStart`
            (:`Update`
              (`self.FinishAISpawn`)
              (`KismetSystemLibrary.PrintString` "播放结束动画"))))))))

(event `SpawnNext`
  (bind (_spwanactor _needwaittime _number) (break `/Game/AISpwaner/S_SpawnInfo` (`|GetArrayItem` (`self.SpawnInfos`) (`self.CurrentSpawnIndex`))))
  (if (>= (- (`KismetArrayLibrary.Array_Length` (`self.SpawnInfos`)) 1) (`self.CurrentSpawnIndex`))
    (for _index (range _number)
      (bind _output (`|GetArrayItem` (`self.SpwanLocations`) _index))
      (bind _returnvalue (`SceneComponent.K2_GetComponentLocation` _output))
      (bind _returnvalue_2 (`|SpawnActorFromClass` _spwanactor (`KismetMathLibrary.MakeTransform` _returnvalue (`SceneComponent.K2_GetComponentRotation` _output)) "Undefined" "MultiplyWithRoot" null null))
      (`GameplayStatics.PlaySoundAtLocation` "/Game/CombatSystem/CourseFiles/SoundFX/A_Character_Heal01.A_Character_Heal01" _returnvalue (struct) 1.0 1.0 0.0 null null null null)
      (`AITask_MoveTo.AIMoveTo` (`AIBlueprintHelperLibrary.GetAIController` _returnvalue_2) (`SceneComponent.K2_GetComponentLocation` (`self.DoorPosition`)) _returnvalue_2))
    (set `self.CurrentSpawnIndex` (+ (`self.CurrentSpawnIndex`) 1))
    (`self.StartWork`)
    (else
      (goto _label))))

(fn `UserConstructionScript`)