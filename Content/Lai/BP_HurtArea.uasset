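; BP_HurtArea is a damage area that hurts combat characters entering its box and periodically spawns a damage test actor, apparently for testing hit handling.
; On box overlap, a BP_CombatCharacter takes point damage using the sweep's impact normal, with that character's own main weapon passed as the damage causer.
; A looping three-second timer started at BeginPlay spawns BP_ShooteDamageTest at the area's transform.
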(event `self.ReceiveBeginPlay`
  (`KismetSystemLibrary.K2_SetTimerDelegate` (delegate `CustomEvent`) 3.0 true))

(event `CustomEvent`
  (`|SpawnActorFromClass` "/Game/Lai/BP_ShooteDamageTest.BP_ShooteDamageTest_C" (`self.GetTransform`) "Undefined" "MultiplyWithRoot" null null))

(event `self.Box.OnComponentBeginOverlap`
  (params (OverlappedComponent :type "PrimitiveComponent Object Reference") (OtherActor :type "Actor Object Reference") (OtherComp :type "PrimitiveComponent Object Reference") (OtherBodyIndex :type Integer) (bFromSweep :type Boolean) (SweepResult :type "HitResult Structure (by ref)"))
  (bind _asbp_combat_character (cast `/Game/CombatSystem/Blueprints/BP_CombatCharacter` OtherActor))
  (`GameplayStatics.ApplyPointDamage` OtherActor 1.0 (`.ImpactNormal` (`GameplayStatics.BreakHitResult` SweepResult)) SweepResult (`self.GetInstigatorController`) (`/Game/CombatSystem/Blueprints/Components/BP_CombatComponent.GetMainWeapon` (`/Game/CombatSystem/Blueprints/BP_CombatCharacter.CombatComponent` _asbp_combat_character))))

(fn `UserConstructionScript`)