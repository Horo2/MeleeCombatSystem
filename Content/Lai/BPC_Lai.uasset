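; Player combat component for a hold-and-release Iai sword dash.
; Tick tracks charge, sped up during a quick-stance window, and drives readiness visuals.
; A charged release plays a montage whose notifies bound a sphere sweep damaging each actor once; move functions dash along camera facing through pawns.
; Link time slows the game, letting CheckLinkAttack trigger an invincible follow-up that curve-lerps the player to the locked target.
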(event `self.ReceiveBeginPlay`
  (`self.SetComponentTickEnabled` false))

(event `HoldLai`
  (bind _bp_player (`self.BP_Player`))
  (`AnimInstance.Montage_Stop` (`SkeletalMeshComponent.GetAnimInstance` (`Character.Mesh` _bp_player)) 0.1 null)
  (`/Game/CombatSystem/Blueprints/BP_CombatCharacter.ResetAttack` _bp_player)
  (`/Game/CombatSystem/Blueprints/Interface/CombatBPI.ResetCombat` _bp_player)
  (set `self.LaiHold` true)
  (set `/Game/CombatSystem/Blueprints/BP_CombatCharacter.CanInputMove` false (`self.BP_Player`))
  (if (`self.IsRateTime`)
    (set `self.LaiPlayRate` 2.0)
    (else
      (set `self.LaiPlayRate` 1.0))))

(event `RelessLai`
  (bind _returnvalue (`/Game/CombatSystem/Blueprints/Components/BP_CombatComponent.GetMainWeapon` (`/Game/CombatSystem/Blueprints/BP_CombatCharacter.CombatComponent` (`self.BP_Player`))))
  (set `self.LaiPlayRate` 1.0)
  (set `self.LaiHold` false)
  (if (`self.CanLai`)
    (bind _notifyname (`|PlayMontage` (`self.PlayerMesh`) "/Game/Lai/AS_Combo_Attack_02_01_Seq_Montage1.AS_Combo_Attack_02_01_Seq_Montage1" 1.0 0.0 "HoldStart")
      (:`OnCompleted`
        (if (not (`self.LaiHold`))
          (`CharacterMovementComponent.SetMovementMode` (`self.CharacterMovement`) "MOVE_Walking" 0 :!label _label)
          (set `/Game/CombatSystem/Blueprints/BP_CombatCharacter.CanInputMove` true (`self.BP_Player`))
          (set `self.IsRateTime` false)))
      (:`OnInterrupted`
        (`KismetSystemLibrary.PrintString` "Hello")
        (goto _label))
      (:`OnNotifyBegin`
        (if (== _notifyname "StartLai")
          (set `self.StartLaiLoc` (`Actor.K2_GetActorLocation` (`self.BP_Player`)))
          (elif (== _notifyname "EndLai")
            ;[1 1 1] 检测路径上的所有敌人
            (bind _output_get (set `self.EndLaiLoc` (`Actor.K2_GetActorLocation` (`self.BP_Player`))))
            (bind _outhits (`KismetSystemLibrary.SphereTraceMultiForObjects` :`Start` (`self.StartLaiLoc`) :`End` _output_get :`Radius` 80.0 :`ObjectTypes` (`|MakeArray` "ObjectTypeQuery3" :!type "EObjectTypeQuery Enum") :`DrawDebugType` "ForDuration"))
            ;[1 1 1] 保证每个物体 只受一次伤害
            (for _array_element _outhits
              (`BlueprintMapLibrary.Map_Add` (`self.HitActors`) (`.HitActor` (`GameplayStatics.BreakHitResult` _array_element)) _array_element))
            ;[1 1 1] 施加伤害
            (bind _values (`BlueprintMapLibrary.Map_Values` (`self.HitActors`)))
            (for _array_element_2 _values
              (bind (_bblockinghit _binitialoverlap _time _distance _location _impactpoint _normal _impactnormal _physmat _hitactor) (`GameplayStatics.BreakHitResult` _array_element_2))
              (`GameplayStatics.ApplyPointDamage` _hitactor (`KismetMathLibrary.SelectFloat` 100.0 50.0 (`self.ShoundIntoLinkTime`)) _impactnormal _array_element_2 (`Actor.GetInstigatorController` _returnvalue) _returnvalue))))))
    (else
      (`CharacterMovementComponent.SetMovementMode` (`self.CharacterMovement`) "MOVE_Walking" 0)
      (set `/Game/CombatSystem/Blueprints/BP_CombatCharacter.CanInputMove` true (`self.BP_Player`))
      (set `self.IsRateTime` false))))

(event `ResetRateTime`
  (`KismetSystemLibrary.K2_ClearAndInvalidateTimerHandle` (`self.NewVar_0`))
  (bind _returnvalue (`KismetSystemLibrary.K2_SetTimerDelegate` (delegate `CustomEvent`) 0.5))
  (set `self.NewVar_0` _returnvalue))

(event `CustomEvent`
  (set `self.IsRateTime` false))

(event `self.ReceiveTick`
  (params (DeltaSeconds :type "Float (single-precision)"))
  (bind _canlaieffect (`self.CanLaiEffect`))
  (bind _returnvalue (`KismetMathLibrary.FClamp` (`CurveFloat.GetFloatValue` (`self.MoveCurve`) (`self.CurrentMoveTime`))))
  (`|ExecutionSequence`
    (:`then_0`
      (if (`self.LaiHold`)
        (bind _output_get (set `self.CurrentHoldTime` (+ (`self.CurrentHoldTime`) (`GameplayStatics.GetWorldDeltaSeconds`))))
        (set `self.CanLai` (>= _output_get (/ (`self.NeedHoldTime`) (`self.LaiPlayRate`))))
        (else
          (set `self.CurrentHoldTime` 0.0)
          (set `self.CanLai` false)))
      (`KismetMaterialLibrary.SetVectorParameterValue` "/Game/Lai/MC_Swoard.MC_Swoard" "Vector" (`KismetMathLibrary.SelectColor` (struct :`R` 3.0 :`A` 1.0) (struct) (`self.CanLai`)))
      (`/Engine/EditorBlueprintResources/StandardMacros.IsValid` _canlaieffect
        (:`Is Valid`
          (`SceneComponent.SetVisibility` _canlaieffect (`self.CanLai`) false))))
    (:`then_1`
      (if (`self.IsRateTime`)
        (set `self.Timming` (- (`self.Timming`) (`GameplayStatics.GetWorldDeltaSeconds`)))
        (`KismetMaterialLibrary.SetScalarParameterValue` "/Game/Lai/MC_Swoard.MC_Swoard" "Enable" 1.0)
        (else
          (set `self.Timming` 0.5)
          (`KismetMaterialLibrary.SetScalarParameterValue` "/Game/Lai/MC_Swoard.MC_Swoard" "Enable"))))
    (:`then_2`
      (if (`self.NeedLinkMove`)
        (`Actor.K2_SetActorLocation` (`self.BP_Player`) (`KismetMathLibrary.VLerp` (`self.StartMoveLoc`) (`self.TargetMoveLoc`) _returnvalue) false false)
        (set `self.CurrentMoveTime` (+ (`self.CurrentMoveTime`) (`GameplayStatics.GetWorldDeltaSeconds`)))
        (if (>= _returnvalue 1.0)
          (set `self.NeedLinkMove` false))))))

(event `LinkAttack`
  (`|PlayMontage` (`self.PlayerMesh`) (`self.LinkAttackmongtage`)
    (:`then`
      (set `self.Invincent` true))
    (:`OnCompleted`
      (set `self.Invincent` false :!label _label_2)
      (`/Game/CombatSystem/Blueprints/BP_CombatCharacter.ResetCombat` (`self.BP_Player`)))
    (:`OnInterrupted`
      (goto _label_2))))

(event `LinkActtackMove`)

(fn `BreakMontage`
  (`Character.StopAnimMontage` (`self.BP_Player`) (`self.LaiMontages`))
  (set `self.CanLai` false)
  (set `self.LaiHold` false)
  (set `self.IsRateTime` false)
  (`CharacterMovementComponent.SetMovementMode` (`self.CharacterMovement`) "MOVE_Walking" 0))

(fn `CheckLinkAttack`
  (returns (Invincent :type Boolean) (Rst :type Boolean))
  (bind _returnvalue (`Actor.K2_GetActorLocation` (`TargetSystemComponent.GetLockedOnTargetActor` (`self.Target Component`))))
  (bind (_returnvalue_x _returnvalue_y) (`KismetMathLibrary.BreakVector` (- _returnvalue (`Actor.K2_GetActorLocation` (`self.BP_Player`)))))
  (`/Engine/EditorBlueprintResources/StandardMacros.IsValid` (`TargetSystemComponent.GetLockedOnTargetActor` (`self.Target Component`))
    (:`Is Valid`
      (if (`self.LinkTimeing`)
        (`KismetSystemLibrary.K2_ClearAndInvalidateTimerHandle` (`self.LinkTimgingTimer`))
        (`self.StopLinkTime`)
        (`self.LinkAttack`)
        (set `self.StartMoveLoc` (`Actor.K2_GetActorLocation` (`self.BP_Player`)))
        (set `self.TargetMoveLoc` (- _returnvalue (`KismetMathLibrary.Normal` (`KismetMathLibrary.MakeVector` _returnvalue_x _returnvalue_y))))
        (set `self.NeedLinkMove` true)
        (set `self.CurrentMoveTime` 0.0)
        (return (`self.Invincent`) true)
        (else
          _)))
    (:`Is Not Valid`
      _))
  (`self.StopLinkTime`)
  (return (`self.Invincent`) false))

(fn `CheckLinkTime`
  (bind _slowrate (`self.SlowRate`))
  (if (`self.ShoundIntoLinkTime`)
    (`GameplayStatics.SetGlobalTimeDilation` (/ 1.0 _slowrate))
    (set `self.LinkTimeing` true))
  (set `self.ShoundIntoLinkTime` false)
  (bind _returnvalue (`KismetSystemLibrary.K2_SetTimerDelegate` (`|CreateDelegate` :!event `StopLinkTime`) (/ (`self.LinkTimePresient`) _slowrate)))
  (set `self.LinkTimgingTimer` _returnvalue))

(fn `EndMove`
  (`PrimitiveComponent.SetCollisionResponseToChannel` (`Character.CapsuleComponent` (`self.BP_Player`)) "ECC_Pawn" "ECR_Block"))

(fn `Init`
  (params (BP_Player :type "/Game/CombatSystem/Blueprints/BP_CombatCharacter Object Reference") (TargetComponent :type "TargetSystemComponent Object Reference") (CanLaiEffect :type "NiagaraComponent Object Reference"))
  (set `self.CanLaiEffect` CanLaiEffect)
  (set `self.Target Component` TargetComponent)
  (bind _output_get (set `self.BP_Player` BP_Player))
  (add `/Game/CombatSystem/Blueprints/BP_CombatCharacter.ED_HoldLai` _output_get (`|CreateDelegate` :!event `HoldLai`))
  (add `/Game/CombatSystem/Blueprints/BP_CombatCharacter.ED_RelessLai` _output_get (`|CreateDelegate` :!event `RelessLai`))
  (set `self.PlayerMesh` (`Character.Mesh` _output_get))
  (set `self.CharacterMovement` (`Character.CharacterMovement` _output_get))
  (`self.SetComponentTickEnabled` true))

(fn `LaiMove`
  (params (Speed :type "Float (double-precision)"))
  (bind _returnvalue (* (`self.MoveDir`) Speed))
  (`Actor.K2_AddActorWorldOffset` (`self.BP_Player`) _returnvalue true false)
  (`SceneComponent.K2_AddWorldOffset` (`self.ShanEffect`) (/ _returnvalue (2.0 2.0 2.0)) false false))

(fn `StartMove`
  (bind _shaneffect (`self.ShanEffect`))
  (bind _bp_player (`self.BP_Player`))
  (bind (_returnvalue_x _returnvalue_y) (`KismetMathLibrary.BreakVector` (`SceneComponent.GetForwardVector` (`PlayerCameraManager.TransformComponent` (`GameplayStatics.GetPlayerCameraManager` 0)))))
  (bind (_returnvalue_x_2 _returnvalue_y_2) (`KismetMathLibrary.BreakVector` (`SceneComponent.GetForwardVector` (`PlayerCameraManager.TransformComponent` (`GameplayStatics.GetPlayerCameraManager` 0)))))
  (bind _returnvalue (`KismetMathLibrary.MakeRotFromX` (`KismetMathLibrary.MakeVector` _returnvalue_x _returnvalue_y)))
  (`PrimitiveComponent.SetCollisionResponseToChannel` (`Character.CapsuleComponent` (`self.BP_Player`)) "ECC_Pawn" "ECR_Overlap")
  (`Actor.K2_SetActorRotation` _bp_player _returnvalue false)
  (`/Engine/EditorBlueprintResources/StandardMacros.IsValid` _shaneffect
    (:`Is Valid`
      (`self.K2_DestroyComponent` _shaneffect))
    (:`Is Not Valid`
      _))
  (bind _returnvalue_2 (`NiagaraFunctionLibrary.SpawnSystemAtLocation` "/Game/Lai/JuHe_VFX/NS_juheyishan_SwordPierce_Lv3.NS_juheyishan_SwordPierce_Lv3" (`Actor.K2_GetActorLocation` _bp_player) _returnvalue))
  (set `self.ShanEffect` _returnvalue_2)
  (set `self.MoveDir` (`KismetMathLibrary.Normal` (`KismetMathLibrary.MakeVector` _returnvalue_x_2 _returnvalue_y_2))))

(fn `StopLinkTime`
  (`GameplayStatics.SetGlobalTimeDilation` 1.0)
  (set `self.LinkTimeing` false))