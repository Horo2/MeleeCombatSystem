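; Base player character that handles Enhanced Input movement and look, forwards spawn and control keys to its controller, and offers preset camera shakes.
; Each tick it scores nearby BP_E1 enemies by angle and distance, though MaxScore never updates, so the last candidate wins.
; The controller stores that focus enemy, and the character smoothly yaws toward it while attacking, unless traces find an enemy above, or below while falling.
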(event Custom|MyControllerPossessed
  (params (Normal :type Boolean))
  (if Normal
    _
    (else
      _))
  (CallFunction|InitInput)
  (Variables|Default|SetMoveAxis "")
  (Collision|SetCollisionProfileName (Variables|Default|GetCapsuleComponent) "Pawn" true :!class /Script/Engine.PrimitiveComponent))

(event Custom|ClearToggleLock
  (Variables|/Game/WorkSpace/Game/MyPlayerController.MyPlayerController_C|SetToggleLock (stale Input|EnhancedActionEvents|EnhancedInputActionIA_Space _as_my_player_controller) false))

(event Input|EnhancedActionEvents|EnhancedInputActionIA_Look
  (params (ActionValue :type Vector%202D%20Structure) (ElapsedSeconds :type Float%20%28double-precision%29) (TriggeredSeconds :type Float%20%28double-precision%29) (InputAction :type Input%20Action%20Object%20Reference :default "/Game/ThirdPerson/Input/Actions/IA_Look.IA_Look"))
  (bind (_x _y) (Math|Vector2D|BreakVector2D ActionValue))
  (Pawn|Input|AddControllerYawInput (* _x (Variables|Default|GetYawSpeed)))
  (Pawn|Input|AddControllerPitchInput (* _y (Variables|Default|GetPitchSpeed))))

(event Input|EnhancedActionEvents|EnhancedInputActionIA_Move
  (params (ActionValue :type Vector%202D%20Structure) (ElapsedSeconds :type Float%20%28double-precision%29) (TriggeredSeconds :type Float%20%28double-precision%29) (InputAction :type Input%20Action%20Object%20Reference :default "/Game/ThirdPerson/Input/Actions/IA_Move.IA_Move"))
  (:Triggered
    (Variables|Default|SetMoveAxis ActionValue)
    (Variables|Default|SetSprintState (>= TriggeredSeconds (Variables|NeedSet|GetSprintThreshold))))
  (:Completed
    (Variables|Default|SetMoveAxis "")))

(event Input|EnhancedActionEvents|EnhancedInputActionIA_Space
  (params (ActionValue :type Boolean) (ElapsedSeconds :type Float%20%28double-precision%29) (TriggeredSeconds :type Float%20%28double-precision%29) (InputAction :type Input%20Action%20Object%20Reference :default "/Game/ThirdPerson/Input/Actions/IA_Space.IA_Space"))
  (:Started
    (bind _as_my_player_controller (CallFunction|GetMyController))
    (if (not (Variables|/Game/WorkSpace/Game/MyPlayerController.MyPlayerController_C|GetToggleLock _as_my_player_controller))
      (Variables|/Game/WorkSpace/Game/MyPlayerController.MyPlayerController_C|SetToggleLock _as_my_player_controller true)
      (Default|DefaultControlPlayer _as_my_player_controller)
      (Utilities|Time|SetTimerbyEvent (delegate Custom|ClearToggleLock) 0.2))))

(event Input|EnhancedActionEvents|EnhancedInputActionIA_E
  (params (ActionValue :type Boolean) (ElapsedSeconds :type Float%20%28double-precision%29) (TriggeredSeconds :type Float%20%28double-precision%29) (InputAction :type Input%20Action%20Object%20Reference :default "/Game/ThirdPerson/Input/Actions/IA_E.IA_E"))
  (:Started
    (bind _as_my_player_controller (CallFunction|GetMyController))
    (Default|SpecSpawnPlayer _as_my_player_controller true)))

(event Input|EnhancedActionEvents|EnhancedInputActionIA_Q
  (params (ActionValue :type Boolean) (ElapsedSeconds :type Float%20%28double-precision%29) (TriggeredSeconds :type Float%20%28double-precision%29) (InputAction :type Input%20Action%20Object%20Reference :default "/Game/ThirdPerson/Input/Actions/IA_Q.IA_Q"))
  (:Started
    (bind _as_my_player_controller (CallFunction|GetMyController))
    (Default|SpecSpawnPlayer _as_my_player_controller false)))

(event EventBeginPlay
  (|CallParentFunction))

(event EventTick
  (params (DeltaSeconds :type Float%20%28single-precision%29))
  (Utilities|FlowControl|Sequence
    (:then_0
      (bind (_seek_ _seekenemy) (CallFunction|SeekEnemy "/Game/WorkSpace/Character/Characters/Enemy/BP_E1.BP_E1_C" 0.3 0.7 2.5e+03))
      (CallFunction|SetFocusEnemy _seekenemy)
      (if _seek_
        (if (Default|IsAttacking (Variables|Default|GetActionComponent))
          (CallFunction|SetActorRotationtoFocusTarget (CallFunction|GetFocusEnemy)))))))

(event EventOnLanded
  (params (Hit :type Hit%20Result%20Structure%20%28by%20ref%29))
  (Default|FindActionHandlerExec (Variables|Default|GetActionComponent) "NewEnumerator14"))

(event EventUnpossessed
  (params (OldController :type Controller%20Object%20Reference)))

(event EventPossessed
  (params (NewController :type Controller%20Object%20Reference))
  (Components|SkeletalMesh|AnimationBlueprintLinking|LinkAnimClassLayers (Variables|Character|GetMesh) (Variables|Default|GetAnim%20Layer%20In%20Class)))

(event Input|KeyboardEvents|DebugKey1
  (params (Key :type Key%20Structure :default "None") (ActionValue :type Input%20Action%20Value%20Structure))
  (:Pressed
    (Transformation|SetActorLocation "2811.000000,2533.000000,50.000000" false false)
    (bind _returnvalue (Actor|GetActorOfClass "/Game/WorkSpace/Character/Characters/Enemy/BP_E1.BP_E1_C"))
    (Transformation|SetActorLocation _returnvalue "2977.000000,2505.000000,109.000000" false false)
    (Transformation|SetActorRotation _returnvalue "0.000000,179.000000,0.000000")))

(fn ConstructionScript
  (|CallParentFunction))

(fn Damage
  (params (HitSource :type BP%20Base%20Character%20Object%20Reference) (HitDetail :type F%20Hit%20Detail%20Structure))
  (return false))

(fn SeekEnemy
  (params (ActorClassFilter :type Object%20Class%20Reference) (DistanceWeight :type Float%20%28double-precision%29) (AngleWeight :type Float%20%28double-precision%29) (Distance :type Float%20%28double-precision%29))
  (bind (_outactors _returnvalue) (Collision|SphereOverlapActors (Transformation|GetActorLocation) Distance (Utilities|Array|MakeArray "ObjectTypeQuery3") ActorClassFilter (Utilities|Array|MakeArray self)))
  (if _returnvalue
    (bind (_seek_ _seekenemy) (CallFunction|ChooseEnemy _outactors DistanceWeight AngleWeight Distance))
    (return _seek_ _seekenemy)))

(fn ChooseEnemy
  (params (Actors :type Array%20of%20Actor%20Object%20References) (DistanceWeight :type Float%20%28double-precision%29) (DirectionWeight :type Float%20%28double-precision%29) (SeekDistance :type Float%20%28double-precision%29))
  (LocalVariables|SetMaxScore 0.0)
  (for _array_element Actors
    (bind _asbp_base_character (Utilities|Casting|CastToBP_BaseCharacter _array_element))
    (bind _score (CallFunction|CalcEnemyFocusScore _array_element DistanceWeight DirectionWeight SeekDistance))
    (if (>= _score (LocalVariables|GetMaxScore))
      (LocalVariables|SetFocusEnemy _asbp_base_character)))
  (Utilities|IsValid (LocalVariables|GetFocusEnemy)
    (:Is%20Valid
      (return true (LocalVariables|GetFocusEnemy)))
    (:Is%20Not%20Valid
      (return false 0))))

(fn CalcPlayertoEnemyAngle
  (params (Actor :type Actor%20Object%20Reference))
  (Utilities|IsValid Actor
    (:Is%20Valid
      (return (* (/ 1.8e+02 3.14) (Math|Trig|Acos(Degrees) (Math|Vector|DotProduct (Transformation|GetActorForwardVector) (Math|Vector|Normalize (- (Transformation|GetActorLocation Actor) (Transformation|GetActorLocation))))))))
    (:Is%20Not%20Valid
      (return -1.0))))

(fn CalcEnemyFocusScore
  (params (Actor :type Actor%20Object%20Reference) (DistanceWeight :type Float%20%28double-precision%29) (AngleWeight :type Float%20%28double-precision%29) (SeekDistance :type Float%20%28double-precision%29))
  (Utilities|IsValid Actor
    (:Is%20Valid
      (bind _angle (CallFunction|CalcPlayertoEnemyAngle Actor))
      (return (+ (* AngleWeight (- 1.0 (Math|Float|Clamp(Float) (/ _angle 1.8e+02)))) (* DistanceWeight (- 1.0 (Math|Float|Clamp(Float) (/ (Math|Vector|Distance(Vector) (Transformation|GetActorLocation) (Transformation|GetActorLocation Actor)) SeekDistance)))))))
    (:Is%20Not%20Valid
      (return 0.0))))

(fn SetFocusEnemy
  (params (FocusActor :type BP%20Base%20Character%20Object%20Reference))
  (bind _as_my_player_controller (CallFunction|GetMyController))
  (Variables|/Game/WorkSpace/Game/MyPlayerController.MyPlayerController_C|SetFocusEnemy _as_my_player_controller FocusActor))

(fn GetFocusEnemy
  (bind _as_my_player_controller (CallFunction|GetMyController))
  (return (Variables|/Game/WorkSpace/Game/MyPlayerController.MyPlayerController_C|GetFocusEnemy _as_my_player_controller)))

(fn SetActorRotationtoFocusTarget
  (params (FocusTarget :type Actor%20Object%20Reference))
  (bind _returnvalue (Transformation|GetActorRotation))
  (bind (_roll _pitch) (Math|Rotator|BreakRotator _returnvalue))
  (if (not (CallFunction|DontRotatortoTarget))
    (bind _hasenemy (CallFunction|CheckPlayerVerticleAreaHasEnemy))
    (if (not _hasenemy)
      (Transformation|SetActorRotation (Math|Interpolation|RInterpTo _returnvalue (Math|Rotator|MakeRotator _roll _pitch (.yaw (Math|Rotator|FindLookatRotation (Transformation|GetActorLocation) (Transformation|GetActorLocation FocusTarget)))) (Utilities|Time|GetWorldDeltaSeconds) (Variables|NeedSet|GetRotatorToTargetSpeed))))))

(fn PlayCameraEffect
  (params (SizePreset :type E_SizePreset%20Enum :default "NewEnumerator0") (CartonPreset :type E_SizePreset%20Enum :default "NewEnumerator0") (UseCustom :type Boolean) (CustomClass :type Camera%20Shake%20Base%20Class%20Reference) (InnerRadius :type Float%20%28double-precision%29) (OuterRadius :type Float%20%28double-precision%29) (Falloff :type Float%20%28double-precision%29))
  (bind _returnvalue (Transformation|GetActorLocation))
  (bind _camerashakepreset (Variables|Default|GetCameraShakePreset))
  (bind (_value _returnvalue_2) (Utilities|Map|Find _camerashakepreset SizePreset))
  (Utilities|FlowControl|Sequence
    (:then_0
      (if UseCustom
        (Camera|PlayWorldCameraShake CustomClass _returnvalue InnerRadius OuterRadius Falloff)
        (elif _returnvalue_2
          (Camera|PlayWorldCameraShake _value _returnvalue InnerRadius OuterRadius Falloff))))
    (:then_1
      (if (.ReturnValue (Utilities|Map|Find (Variables|Default|GetCartonPreset) CartonPreset))
        (Development|PrintString "to do some thing")))))

(fn InitInput
  (bind _asplayer_controller (Utilities|Casting|CastToPlayerController (Pawn|GetController)))
  (Utilities|IsValid (PlayerController|LocalPlayerSubsystems|GetEnhancedInputLocalPlayerSubsystem _asplayer_controller)
    (:Is%20Valid
      (Input|AddMappingContext (PlayerController|LocalPlayerSubsystems|GetEnhancedInputLocalPlayerSubsystem _asplayer_controller) "/Game/ThirdPerson/Input/IMC_Default.IMC_Default" 0 "(bIgnoreAllPressedKeysUntilRelease=True,bForceImmediately=False,bNotifyUserSettings=False)"))))

(fn DontRotatortoTarget
  (return false))

(fn CheckPlayerVerticleAreaHasEnemy
  (bind _returnvalue (Transformation|GetActorLocation))
  (bind _returnvalue_2 (Transformation|GetActorLocation))
  (Utilities|FlowControl|Sequence
    (:then_0
      (bind (_outhit _returnvalue_3) (Collision|LineTraceByChannel _returnvalue_2 (+ _returnvalue_2 (* (Transformation|GetActorUpVector) 2000)) "TraceTypeQuery2" false 0 "ForOneFrame"))
      (if _returnvalue_3
        (if (Actor|ActorHasTag (.HitActor (Collision|BreakHitResult _outhit)) "Enemy")
          (Transformation|AddActorLocalOffset (.HitActor (Collision|BreakHitResult _outhit)) (* (Transformation|GetActorForwardVector) 10) false false)
          (return true))))
    (:then_1
      (if (AI|Components|NavMovement|IsFalling (Variables|Character|GetCharacterMovement))
        (bind (_outhit_2 _returnvalue_4) (Collision|CapsuleTraceByChannel _returnvalue (+ _returnvalue (* (Transformation|GetActorUpVector) -500)) 5e+01 1e+01 "TraceTypeQuery2" false 0 "ForOneFrame"))
        (if _returnvalue_4
          (if (Actor|ActorHasTag (.HitActor (Collision|BreakHitResult _outhit_2)) "Enemy")
            (return true)))))))

(fn GetFocusTarget
  (bind _focusenemy (CallFunction|GetFocusEnemy))
  (return (Utilities|IsValid _focusenemy) _focusenemy))

(fn GetSpringArmInfo
  (return "0, 0, 0" 0.0))