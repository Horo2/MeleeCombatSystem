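; BP_P3 is a playable character Blueprint that maps Enhanced Input to combat actions run by its ActionComponent.
; Shift picks a directional or stationary action, snapping rotation to the move direction when there is input.
; Mouse attacks choose variants by falling state and any active Shift action, while F varies by falling state.
; F release and landing are forwarded to the current handler, and DontRotatorToTarget flags actions that skip target-facing.
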(event `EnhancedInput|/Game/ThirdPerson/Input/Actions/IA_Shift`
  (params (ActionValue :type Boolean) (ElapsedSeconds :type "Float (double-precision)") (TriggeredSeconds :type "Float (double-precision)") (InputAction :type "InputAction Object Reference" :default "/Game/ThirdPerson/Input/Actions/IA_Shift.IA_Shift"))
  (bind _actioncomponent (`self.ActionComponent`))
  (:`Started`
    (if (`KismetMathLibrary.IsZero2D` (`self.MoveAxis`))
      (`/Game/WorkSpace/Character/Characters/Action/ActionComponent.FindActionHandlerExec` _actioncomponent "NewEnumerator16")
      (else
        (`self.K2_SetActorRotation` (`KismetMathLibrary.Conv_VectorToRotator` (`self.CalcDirectionVector`)))
        (`/Game/WorkSpace/Character/Characters/Action/ActionComponent.FindActionHandlerExec` _actioncomponent "NewEnumerator15")))))

(event `EnhancedInput|/Game/ThirdPerson/Input/Actions/IA_LeftMouse`
  (params (ActionValue :type Boolean) (ElapsedSeconds :type "Float (double-precision)") (TriggeredSeconds :type "Float (double-precision)") (InputAction :type "InputAction Object Reference" :default "/Game/ThirdPerson/Input/Actions/IA_LeftMouse.IA_LeftMouse"))
  (bind _actioncomponent (`self.ActionComponent`))
  (bind _actioncomponent_2 (`self.ActionComponent`))
  (:`Started`
    (if (`NavMovementComponent.IsFalling` (`self.CharacterMovement`))
      (if (or (`/Game/WorkSpace/Character/Characters/Action/ActionComponent.CurrentIsAttacking` _actioncomponent "NewEnumerator15") (`/Game/WorkSpace/Character/Characters/Action/ActionComponent.CurrentIsAttacking` _actioncomponent "NewEnumerator16"))
        (`/Game/WorkSpace/Character/Characters/Action/ActionComponent.FindActionHandlerExec` _actioncomponent "NewEnumerator19")
        (else
          (`/Game/WorkSpace/Character/Characters/Action/ActionComponent.FindActionHandlerExec` _actioncomponent "NewEnumerator5")))
      (elif (or (`/Game/WorkSpace/Character/Characters/Action/ActionComponent.CurrentIsAttacking` _actioncomponent_2 "NewEnumerator15") (`/Game/WorkSpace/Character/Characters/Action/ActionComponent.CurrentIsAttacking` _actioncomponent_2 "NewEnumerator16"))
        (`/Game/WorkSpace/Character/Characters/Action/ActionComponent.FindActionHandlerExec` _actioncomponent_2 "NewEnumerator17")
        (else
          (`/Game/WorkSpace/Character/Characters/Action/ActionComponent.FindActionHandlerExec` _actioncomponent_2 "NewEnumerator0"))))))

(event `EnhancedInput|/Game/ThirdPerson/Input/Actions/IA_RightMouse`
  (params (ActionValue :type Boolean) (ElapsedSeconds :type "Float (double-precision)") (TriggeredSeconds :type "Float (double-precision)") (InputAction :type "InputAction Object Reference" :default "/Game/ThirdPerson/Input/Actions/IA_RightMouse.IA_RightMouse"))
  (bind _actioncomponent (`self.ActionComponent`))
  (bind _actioncomponent_2 (`self.ActionComponent`))
  (bind _returnvalue (or (`/Game/WorkSpace/Character/Characters/Action/ActionComponent.CurrentIsAttacking` _actioncomponent "NewEnumerator15") (`/Game/WorkSpace/Character/Characters/Action/ActionComponent.CurrentIsAttacking` _actioncomponent "NewEnumerator16")))
  (:`Started`
    (if (`NavMovementComponent.IsFalling` (`self.CharacterMovement`))
      (if _returnvalue
        (`/Game/WorkSpace/Character/Characters/Action/ActionComponent.FindActionHandlerExec` _actioncomponent "NewEnumerator20")
        (else
          (`/Game/WorkSpace/Character/Characters/Action/ActionComponent.FindActionHandlerExec` _actioncomponent "NewEnumerator6")))
      (elif _returnvalue
        (`/Game/WorkSpace/Character/Characters/Action/ActionComponent.FindActionHandlerExec` _actioncomponent_2 "NewEnumerator18")
        (else
          (`/Game/WorkSpace/Character/Characters/Action/ActionComponent.FindActionHandlerExec` _actioncomponent_2 "NewEnumerator1"))))))

(event `EnhancedInput|/Game/ThirdPerson/Input/Actions/IA_F`
  (params (ActionValue :type Boolean) (ElapsedSeconds :type "Float (double-precision)") (TriggeredSeconds :type "Float (double-precision)") (InputAction :type "InputAction Object Reference" :default "/Game/ThirdPerson/Input/Actions/IA_F.IA_F"))
  (bind _actioncomponent (`self.ActionComponent`))
  (:`Started`
    (`/Game/WorkSpace/Character/Characters/Action/ActionComponent.FindActionHandlerExec` _actioncomponent (select `bool` (`NavMovementComponent.IsFalling` (`self.CharacterMovement`)) :`false` "NewEnumerator10" :`true` "NewEnumerator12" :!type "/Game/WorkSpace/Character/Characters/DataType/E_ActionType Enum")))
  (:`Completed`
    (`/Game/WorkSpace/Character/Characters/Action/SingleActionHandler.OnReleased` (`/Game/WorkSpace/Character/Characters/Action/ActionComponent.CurrentHandler` _actioncomponent))))

(event `self.OnLanded`
  (params (Hit :type "HitResult Structure (by ref)"))
  (`/Game/WorkSpace/Character/Characters/Action/SingleActionHandler.OnLanded` (`/Game/WorkSpace/Character/Characters/Action/ActionComponent.CurrentHandler` (`self.ActionComponent`))))

(fn `DontRotatorToTarget`
  (returns (Dont :type Boolean))
  (bind _actioncomponent (`self.ActionComponent`))
  (return (or (`/Game/WorkSpace/Character/Characters/Action/ActionComponent.CurrentIsThis` _actioncomponent "NewEnumerator15" false) (`/Game/WorkSpace/Character/Characters/Action/ActionComponent.CurrentIsThis` _actioncomponent "NewEnumerator16" false) (`/Game/WorkSpace/Character/Characters/Action/ActionComponent.CurrentIsThis` _actioncomponent "NewEnumerator26" false) (`/Game/WorkSpace/Character/Characters/Action/ActionComponent.CurrentIsThis` _actioncomponent "NewEnumerator27" false) (`/Game/WorkSpace/Character/Characters/Action/ActionComponent.CurrentIsThis` _actioncomponent "NewEnumerator28" false) (`/Game/WorkSpace/Character/Characters/Action/ActionComponent.CurrentIsThis` _actioncomponent "NewEnumerator29" false) (`/Game/WorkSpace/Character/Characters/Action/ActionComponent.CurrentIsThis` _actioncomponent "NewEnumerator3" false))))

(fn `UserConstructionScript`
  (`parent.UserConstructionScript`))