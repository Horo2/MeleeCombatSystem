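; BP_BaseEnemy is a base enemy character Blueprint with almost no active logic of its own.
; A capsule hit casts the other actor to BP_BasePlayer and checks whether it is falling, but neither result leads to any action.
; Disconnected nodes would yaw the player to face the enemy during either of two attack states, but they never run.
; BeginPlay, overlap and Tick are unused, and construction only calls the parent.
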(event `self.CapsuleComponent.OnComponentHit`
  (params (HitComponent :type "PrimitiveComponent Object Reference") (OtherActor :type "Actor Object Reference") (OtherComp :type "PrimitiveComponent Object Reference") (NormalImpulse :type "Vector Structure") (Hit :type "HitResult Structure (by ref)"))
  (bind _asbp_base_player (cast `/Game/WorkSpace/Character/Characters/BP_BasePlayer` OtherActor))
  (if (`NavMovementComponent.IsFalling` (`Character.CharacterMovement` _asbp_base_player))
    _))

(fn `UserConstructionScript`
  (`parent.UserConstructionScript`))