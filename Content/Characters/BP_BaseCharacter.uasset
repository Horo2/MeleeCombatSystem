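; Base character Blueprint for melee and thrown-sword combat that spawns an MToon attach actor for its VRM assets on BeginPlay.
; Action phase events forward to handlers looked up in ActionComponent by action type.
; AttackTrace runs box or sphere overlaps; HandleHitActors skips repeat hits until AttackTraceEnd, optionally pulls targets, then calls Damage and the handler's OnHit.
; Helpers cover offsets, sword throwing, enemy box traces and spawning; Damage here is a stub.
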(event `self.ReceiveBeginPlay`
  (bind _returnvalue (`|SpawnActorFromClass` "/VRM4U/Util/Actor/MToonAttachActor.MToonAttachActor_C" (`self.GetTransform`) "Undefined" "MultiplyWithRoot" null null (`self.VRMAsset List`) null))
  (set `/VRM4U/Util/Actor/MToonAttachActor.TargetByActor` self _returnvalue)
  (set `/VRM4U/Util/Actor/MToonAttachActor.bDisableCustomShadowMap` true _returnvalue)
  (`/VRM4U/Util/Actor/MToonAttachActor.initAll` _returnvalue))

(event `/Game/WorkSpace/Character/BPI/BPI_BaseCharacterAllNotify.Action_Exec`
  (params (ActionType :type "/Game/WorkSpace/Character/Characters/DataType/E_ActionType Enum" :default "NewEnumerator0"))
  (bind _value (`/Game/WorkSpace/Character/Characters/Action/ActionComponent.FindActionHandler` (`self.ActionComponent`) ActionType))
  (`/Game/WorkSpace/Character/Characters/Action/SingleActionHandler.Exec` _value ActionType))

(event `/Game/WorkSpace/Character/BPI/BPI_BaseCharacterAllNotify.Action_After_1`
  (params (ActionType :type "/Game/WorkSpace/Character/Characters/DataType/E_ActionType Enum" :default "NewEnumerator0"))
  (bind _value (`/Game/WorkSpace/Character/Characters/Action/ActionComponent.FindActionHandler` (`self.ActionComponent`) ActionType))
  (`/Game/WorkSpace/Character/Characters/Action/SingleActionHandler.After_1` _value ActionType))

(event `/Game/WorkSpace/Character/BPI/BPI_BaseCharacterAllNotify.Action_After_2`
  (params (ActionType :type "/Game/WorkSpace/Character/Characters/DataType/E_ActionType Enum" :default "NewEnumerator0"))
  (bind _value (`/Game/WorkSpace/Character/Characters/Action/ActionComponent.FindActionHandler` (`self.ActionComponent`) ActionType))
  (`/Game/WorkSpace/Character/Characters/Action/SingleActionHandler.After_2` _value ActionType))

(event `/Game/WorkSpace/Character/BPI/BPI_BaseCharacterAllNotify.Action_End`
  (params (ActionType :type "/Game/WorkSpace/Character/Characters/DataType/E_ActionType Enum" :default "NewEnumerator0"))
  (bind _value (`/Game/WorkSpace/Character/Characters/Action/ActionComponent.FindActionHandler` (`self.ActionComponent`) ActionType))
  (`/Game/WorkSpace/Character/Characters/Action/SingleActionHandler.End` _value ActionType))

(event `/Game/WorkSpace/Character/BPI/BPI_BaseCharacterAllNotify.Action_O_1`
  (params (ActionType :type "/Game/WorkSpace/Character/Characters/DataType/E_ActionType Enum" :default "NewEnumerator0"))
  (bind _value (`/Game/WorkSpace/Character/Characters/Action/ActionComponent.FindActionHandler` (`self.ActionComponent`) ActionType))
  (`/Game/WorkSpace/Character/Characters/Action/SingleActionHandler.O_1` _value ActionType))

(event `/Game/WorkSpace/Character/BPI/BPI_BaseCharacterAllNotify.Action_O_2`
  (params (ActionType :type "/Game/WorkSpace/Character/Characters/DataType/E_ActionType Enum" :default "NewEnumerator0"))
  (bind _value (`/Game/WorkSpace/Character/Characters/Action/ActionComponent.FindActionHandler` (`self.ActionComponent`) ActionType))
  (`/Game/WorkSpace/Character/Characters/Action/SingleActionHandler.O_2` _value ActionType))

(event `/Game/WorkSpace/Character/BPI/BPI_BaseCharacterAllNotify.Action_O_3`
  (params (ActionType :type "/Game/WorkSpace/Character/Characters/DataType/E_ActionType Enum" :default "NewEnumerator0"))
  (bind _value (`/Game/WorkSpace/Character/Characters/Action/ActionComponent.FindActionHandler` (`self.ActionComponent`) ActionType))
  (`/Game/WorkSpace/Character/Characters/Action/SingleActionHandler.O_3` _value ActionType))

(event `/Game/WorkSpace/Character/BPI/BPI_BaseCharacterAllNotify.AttackTrace`
  (params (Shape :type "/Game/WorkSpace/Character/Characters/DataType/E_Shape Enum" :default "NewEnumerator0") (BoxSize :type "Vector Structure") (SphereRadius :type "Float (double-precision)") (RelativeOffset :type "Vector Structure") (Debug :type Boolean) (EnableAttach :type Boolean) (AttachOffset :type "Vector Structure") (AttachRate :type "Float (double-precision)") (EnableManyTrigger :type Boolean) (MaxTriggerCount :type Integer) (HitDetail :type "/Game/WorkSpace/Character/Characters/DataType/F_HitDetail Structure"))
  (bind _array (`|MakeArray` "ObjectTypeQuery3" :!type "EObjectTypeQuery Enum"))
  (bind _returnvalue (`self.CalcOffset` true self RelativeOffset))
  (bind _array_2 (`|MakeArray` self :!type "Actor Object Reference"))
  (switch `/Game/WorkSpace/Character/Characters/DataType/E_Shape` Shape
    (:`NewEnumerator0`
      (bind (_outactors _returnvalue_2) (`KismetSystemLibrary.BoxOverlapActors` _returnvalue BoxSize _array (`self.AttackClassFilter`) _array_2))
      (if Debug
        (`KismetSystemLibrary.DrawDebugBox` _returnvalue BoxSize (struct :`R` 0.91463 :`G` 0.44283 :`B` 1.0 :`A` 1.0) (`self.K2_GetActorRotation`) 1.0 1.0))
      (if _returnvalue_2
        (`self.HandleHitActors` _outactors EnableAttach AttachOffset EnableManyTrigger MaxTriggerCount HitDetail AttachRate)))
    (:`NewEnumerator1`
      (bind (_outactors_2 _returnvalue_3) (`KismetSystemLibrary.SphereOverlapActors` _returnvalue SphereRadius _array (`self.AttackClassFilter`) _array_2))
      (if Debug
        (`KismetSystemLibrary.DrawDebugSphere` _returnvalue SphereRadius 12 (struct :`R` 1.0 :`G` 0.540245 :`B` 0.45028 :`A` 1.0) 1.0 1.0))
      (if _returnvalue_3
        (`self.HandleHitActors` _outactors_2 EnableAttach AttachOffset EnableManyTrigger MaxTriggerCount HitDetail AttachRate)))))

(event `/Game/WorkSpace/Character/BPI/BPI_BaseCharacterAllNotify.AttackTraceEnd`
  (`BlueprintSetLibrary.Set_Clear` (`self.HitActions`)))

(event `self.Capsule.OnComponentBeginOverlap`
  (params (OverlappedComponent :type "PrimitiveComponent Object Reference") (OtherActor :type "Actor Object Reference") (OtherComp :type "PrimitiveComponent Object Reference") (OtherBodyIndex :type Integer) (bFromSweep :type Boolean) (SweepResult :type "HitResult Structure (by ref)"))
  (if (`self.ActorHasTag` OtherActor "Char")
    _))

(event `ReceiveSword`
  (params (`Right?` :type Boolean)))

(event `/Game/WorkSpace/Character/BPI/BPI_BaseCharacterAllNotify.AddOffset`
  (params (DeltaRate :type "Float (double-precision)") (Direction :type "/Game/WorkSpace/Character/Characters/DataType/E_4Direction Enum" :default "NewEnumerator0"))
  (bind _returnvalue (`self.GetActorForwardVector`))
  (bind _returnvalue_2 (`self.GetActorRightVector`))
  (bind _returnvalue_3 (* DeltaRate -1.0))
  (`self.K2_AddActorWorldOffset` (select `/Game/WorkSpace/Character/Characters/DataType/E_4Direction` Direction :`NewEnumerator0` (* DeltaRate _returnvalue) :`NewEnumerator1` (* _returnvalue_3 _returnvalue) :`NewEnumerator2` (* _returnvalue_2 DeltaRate) :`NewEnumerator3` (* _returnvalue_3 _returnvalue_2))))

(fn `AttackTraceStart`
  (params (Duration :type "Float (double-precision)"))
  (returns (Return :type Boolean))
  (return true))

(fn `CalcDirectionVector`
  (returns (ReturnValue :type "Vector Structure"))
  (bind (_moveaxis_x _moveaxis_y) (`KismetMathLibrary.BreakVector2D` (`self.MoveAxis`)))
  (bind _returnvalue (`KismetMathLibrary.MakeRotator` 0.0 0.0 (.yaw (`self.GetControlRotation`))))
  (return (+ (* (`KismetMathLibrary.GetForwardVector` _returnvalue) _moveaxis_y) (* (`KismetMathLibrary.GetRightVector` _returnvalue) _moveaxis_x))))

(fn `CalcOffset`
  (params (`AddSelfLocation?` :type Boolean) (Actor :type "Actor Object Reference") (Direction :type "Vector Structure"))
  (returns (ReturnValue :type "Vector Structure"))
  (return (+ (* (`self.GetActorForwardVector` Actor) Direction_X) (* (`self.GetActorRightVector` Actor) Direction_Y) (* (`self.GetActorUpVector` Actor) Direction_Z) (`KismetMathLibrary.SelectVector` (`self.K2_GetActorLocation` Actor) (0.0 0.0 0.0) (`local.AddSelfLocation?`)))))

(fn `Damage`
  (params (HitSource :type "/Game/Characters/BP_BaseCharacter Object Reference") (HitDetail :type "/Game/WorkSpace/Character/Characters/DataType/F_HitDetail Structure"))
  (returns (Hit :type Boolean))
  (return false))

(fn `GetMyController`
  (returns (`As My Player Controller` :type "/Game/WorkSpace/Game/MyPlayerController Object Reference"))
  (bind _as_my_player_controller (`self.As My Player Controller`))
  (`/Engine/EditorBlueprintResources/StandardMacros.IsValid` _as_my_player_controller
    (:`Is Valid`
      (return _as_my_player_controller))
    (:`Is Not Valid`
      (bind _asmy_player_controller (cast `/Game/WorkSpace/Game/MyPlayerController` (`GameplayStatics.GetPlayerController` 0)))
      (bind _output_get (set `self.As My Player Controller` _asmy_player_controller))
      (return _output_get))))

(fn `HandleHitActors`
  (params (HitActors :type "Array of Actor Object Reference") (EnableAttach :type Boolean) (AttachOffset :type "Vector Structure") (EnableManyTrigger :type Boolean) (MaxTriggerCount :type Integer) (HitDetail :type "/Game/WorkSpace/Character/Characters/DataType/F_HitDetail Structure") (AttachRate :type "Float (double-precision)"))
  (for _array_element HitActors
    (if (not (`BlueprintSetLibrary.Set_Contains` (`self.HitActions`) _array_element))
      (`BlueprintSetLibrary.Set_Add` (`self.HitActions`) _array_element)
      (if (`local.EnableAttach`)
        (`self.K2_SetActorLocation` _array_element (`KismetMathLibrary.VInterpTo` (`self.K2_GetActorLocation` _array_element) (`self.CalcOffset` true self AttachOffset) (`GameplayStatics.GetWorldDeltaSeconds`) AttachRate) false false))
      (bind _asbp_base_character (cast `/Game/Characters/BP_BaseCharacter` _array_element))
      (`self.Damage` _asbp_base_character self HitDetail)
      (`/Game/WorkSpace/Character/Characters/Action/SingleActionHandler.OnHit` (`/Game/WorkSpace/Character/Characters/Action/ActionComponent.CurrentHandler` (`self.ActionComponent`)) _asbp_base_character))))

(fn `SetToSafePlace`
  (params (`Leave?` :type Boolean))
  (returns (ReturnValue :type Boolean))
  (bind _asmy_player_controller (cast `/Game/WorkSpace/Game/MyPlayerController` (`GameplayStatics.GetPlayerController` 0)))
  (bind _returnvalue (`/Game/WorkSpace/Game/MyPlayerController.SetActorToSafePlace` _asmy_player_controller self `Leave?`))
  (return _returnvalue))

(fn `SpawnActor`
  (params (Class :type "Actor Class Reference") (UseMeshSocketLocation :type Boolean) (SocketName :type Name) (Location :type "Vector Structure") (UsePawnRotator :type Boolean) (Rotation :type "Rotator Structure"))
  (returns (SpawnActor :type "Actor Object Reference"))
  (bind _returnvalue (`|SpawnActorFromClass` Class (`KismetMathLibrary.MakeTransform` (`KismetMathLibrary.SelectVector` (`SceneComponent.GetSocketLocation` (`self.Mesh`) SocketName) Location UseMeshSocketLocation) (`KismetMathLibrary.SelectRotator` (`self.K2_GetActorRotation`) Rotation UsePawnRotator)) "Undefined" "MultiplyWithRoot" null null))
  (return _returnvalue))

(fn `SpawnSystemAtLocation`
  (params (SystemTemplate :type "NiagaraSystem Object Reference") (Location :type "Vector Structure") (Rotation :type "Rotator Structure") (Scale :type "Vector Structure") (bAutoDestroy :type Boolean))
  (returns (ReturnValue :type "NiagaraComponent Object Reference"))
  (bind _returnvalue (`NiagaraFunctionLibrary.SpawnSystemAtLocation` SystemTemplate Location Rotation Scale bAutoDestroy))
  (return _returnvalue))

(fn `ThrowSword`
  (params (`Right?` :type Boolean) (Duration :type "Float (double-precision)") (Velocity :type "Vector Structure") (Distance :type "Float (double-precision)") (ComeBack :type Boolean) (DeltaRotator :type "Rotator Structure") (ComboBackRate :type "Float (double-precision)") (StaticMesh :type "StaticMesh Object Reference"))
  (returns (ReturnValue :type "/Game/WorkSpace/Character/Characters/P1/Actor/ThrowSwordActor Object Reference"))
  (bind _returnvalue (`|SpawnActorFromClass` "/Game/WorkSpace/Character/Characters/P1/Actor/ThrowSwordActor.ThrowSwordActor_C" (`self.GetTransform`) "Undefined" "MultiplyWithRoot" null null))
  (`/Game/WorkSpace/Character/Characters/P1/Actor/ThrowSwordActor.Fire` _returnvalue `Right?` Velocity Distance Duration ComeBack DeltaRotator self ComboBackRate StaticMesh)
  (bind _output_get (set `self.ThrowWeapon` _returnvalue))
  (return _output_get))

(fn `Trace`
  (params (Start :type "Vector Structure") (End :type "Vector Structure") (HalfSize :type "Vector Structure") (Orientation :type "Rotator Structure") (HitDetail :type "/Game/WorkSpace/Character/Characters/DataType/F_HitDetail Structure"))
  (bind (_outhits _returnvalue) (`KismetSystemLibrary.BoxTraceMulti` Start End HalfSize Orientation "TraceTypeQuery2" false (`|MakeArray` self :!type "Actor Object Reference")))
  (if _returnvalue
    (for _array_element _outhits
      (bind _asbp_base_enemy (cast `/Game/WorkSpace/Character/Characters/BP_BaseEnemy` (`.HitActor` (`GameplayStatics.BreakHitResult` _array_element))))
      (`self.Damage` _asbp_base_enemy self HitDetail))))

(fn `UserConstructionScript`)