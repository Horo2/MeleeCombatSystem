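; BP_ElectricGird is an electric grid hazard that penalizes combat characters and is removed once its linked boxes are destroyed.
; When a BP_CombatCharacter overlaps its Box, it subtracts a fixed amount from one stat in that character's StatsComponent.
; BoxDestroyed counts calls whose BoxID matches the grid's ID and destroys the actor once the count reaches two.
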(event `self.Box.OnComponentBeginOverlap`
  (params (OverlappedComponent :type "PrimitiveComponent Object Reference") (OtherActor :type "Actor Object Reference") (OtherComp :type "PrimitiveComponent Object Reference") (OtherBodyIndex :type Integer) (bFromSweep :type Boolean) (SweepResult :type "HitResult Structure (by ref)"))
  (bind _asbp_combat_character (cast `/Game/CombatSystem/Blueprints/BP_CombatCharacter` OtherActor))
  (bind _output_get (set `self.As BP Combat Character` _asbp_combat_character))
  (`/Game/CombatSystem/Blueprints/Components/BP_StatsComponent.SetCurrentStatValue` (`/Game/CombatSystem/Blueprints/BP_CombatCharacter.StatsComponent` _output_get) "NewEnumerator1" (- (`/Game/CombatSystem/Blueprints/Components/BP_StatsComponent.GetCurrentStatValue` (`/Game/CombatSystem/Blueprints/BP_CombatCharacter.StatsComponent` _asbp_combat_character) "NewEnumerator1") 100.0)))

(fn `BoxDestroyed`
  (params (`Box ID` :type Integer))
  (if (== `Box ID` (`self.ID`))
    (bind _output_get (set `self.Destroyed Box Count` (+ (`self.Destroyed Box Count`) 1)))
    (if (>= _output_get 2)
      (`self.K2_DestroyActor`))))

(fn `UserConstructionScript`)