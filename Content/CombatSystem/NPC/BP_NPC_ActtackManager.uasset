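; Manager actor that limits how many NPCs may attack at once by handing out attack licences.
; From BeginPlay it gathers every BP_NEW_NPC_Character, counts licence holders through their data and behaviour component, and collects the rest as candidates.
; While fewer than three hold a licence, it grants one to a random candidate per pass.
; A delayed reset clears the lists and count, then repeats the pass every 0.2 seconds.
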(event `self.ReceiveBeginPlay`
  (`self.给予攻击许可`))

(event `给予攻击许可`
  (bind _output (`|GetArrayItem` (`self.Can Carry Out Attack NPC`) (`KismetMathLibrary.RandomIntegerInRange` 0 (- (`KismetArrayLibrary.Array_Length` (`self.Can Carry Out Attack NPC`)) 1))))
  (bind _outactors (`GameplayStatics.GetAllActorsOfClass` "/Game/CombatSystem/NPC/BP_NEW_NPC_Character.BP_NEW_NPC_Character_C"))
  (set `self.NPC Character Data` _outactors)
  (for _array_element (`self.NPC Character Data`)
    (if (`/Game/CombatSystem/NPC/C_NPC_DataAndBehaviourManagement_Component.Get NPC Attack LIcence` (`self.GetComponentByClass` _array_element "/Game/CombatSystem/NPC/C_NPC_DataAndBehaviourManagement_Component.C_NPC_DataAndBehaviourManagement_Component_C"))
      (`/Engine/EditorBlueprintResources/StandardMacros.IncrementInt` (`self.已允许攻击的人数`))
      (else
        (`KismetArrayLibrary.Array_Add` (`self.Can Carry Out Attack NPC`) _array_element))))
  (if (< (`self.已允许攻击的人数`) 3)
    (`/Engine/EditorBlueprintResources/StandardMacros.IsValid` _output
      (:`Is Valid`
        (`/Game/CombatSystem/NPC/C_NPC_DataAndBehaviourManagement_Component.Set NPC Attack Licence` (`self.GetComponentByClass` _output "/Game/CombatSystem/NPC/C_NPC_DataAndBehaviourManagement_Component.C_NPC_DataAndBehaviourManagement_Component_C") true)
        (`self.重置给予攻击许可`))
      (:`Is Not Valid`
        (`self.重置给予攻击许可`)))
    (else
      (`self.重置给予攻击许可`))))

(event `重置给予攻击许可`
  (`KismetSystemLibrary.Delay` 0.2)
  (`KismetArrayLibrary.Array_Clear` (`self.Can Carry Out Attack NPC`))
  (set `self.已允许攻击的人数` 0)
  (`KismetArrayLibrary.Array_Clear` (`self.NPC Character Data`))
  (`self.给予攻击许可`))

(fn `UserConstructionScript`)