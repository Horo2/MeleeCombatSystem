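; BP_CombatPlayerController is a player controller that sets up the combat HUD and handles pause menu and door debug-style hotkeys.
; On BeginPlay it creates WB_MainHUD, stores it as MainHUD and adds it to the viewport.
; P adds a new PauseMenu widget and shows the mouse cursor, without pausing the game or changing input mode here.
; G calls DoorOpen on the Door actor returned by GetActorOfClass, with no proximity check.
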(event `Key|P`
  (params (Key :type "Key Structure"))
  (:`Pressed`
    (bind _returnvalue (`|CreateWidget` "/Game/CombatSystem/Menu/PauseMenu.PauseMenu_C"))
    (`UserWidget.AddToViewport` _returnvalue 0)
    (set `PlayerController.bShowMouseCursor` true (`GameplayStatics.GetPlayerController` 0))))

(event `self.ReceiveBeginPlay`
  (bind _returnvalue (`|CreateWidget` "/Game/CombatSystem/UI/WB_MainHUD.WB_MainHUD_C" self))
  (bind _output_get (set `self.MainHUD` _returnvalue))
  (`UserWidget.AddToViewport` _output_get 0))

(event `Key|G`
  (params (Key :type "Key Structure"))
  (:`Pressed`
    (bind _returnvalue (`GameplayStatics.GetActorOfClass` "/Game/CombatSystem/Interaction/Door.Door_C"))
    (`/Game/CombatSystem/Interaction/Door.DoorOpen` _returnvalue)))

(fn `UserConstructionScript`)