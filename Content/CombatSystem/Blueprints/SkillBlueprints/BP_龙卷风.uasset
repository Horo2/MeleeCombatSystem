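; Tornado skill actor that travels forward, damaging and drawing in pawns around it.
; A looping timer sphere-traces for pawns, excluding the releasing actor, then sends damage from its attack data to NPC data components and lerps those targets toward its center.
; Tick spins the mesh and moves the actor by a per-frame step, halting while a forward line trace hits world geometry.
; Both traces leave debug drawing enabled.
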(event `self.ReceiveBeginPlay`
  (`KismetSystemLibrary.K2_SetTimerDelegate` (delegate `自定义事件`) 0.1 true))

(event `自定义事件`
  (bind _returnvalue (`self.K2_GetActorLocation`))
  (bind (_animation _actiondamagemultiplier _actiontoughnessdamagemultiplier _actionscd `_斩切槽消耗` _actionssuperarmor _attacktypeforhitreflection) (break `/Game/CombatSystem/Blueprints/Structs/F_AttackMoves` (`self.Attack Moes Data`)))
  (bind (_outhits _returnvalue_2) (`KismetSystemLibrary.SphereTraceMultiForObjects` _returnvalue _returnvalue 750.0 (`|MakeArray` "ObjectTypeQuery3" :!type "EObjectTypeQuery Enum") false (`|MakeArray` self (`self.Releases Actor`) :!type "Actor Object Reference") "ForDuration"))
  (if _returnvalue_2
    (for _array_element _outhits
      (bind (_bblockinghit _binitialoverlap _time _distance _location _impactpoint _normal _impactnormal _physmat _hitactor) (`GameplayStatics.BreakHitResult` _array_element))
      (bind _returnvalue_3 (`self.GetComponentByClass` _hitactor "/Game/CombatSystem/NPC/C_NPC_DataAndBehaviourManagement_Component.C_NPC_DataAndBehaviourManagement_Component_C"))
      (`/Engine/EditorBlueprintResources/StandardMacros.IsValid` _returnvalue_3
        (:`Is Valid`
          (message `/Game/CombatSystem/NPC/NPC_Interactive_Interface.Create Damage` _returnvalue_3 (* _actiondamagemultiplier (`self.Damage Multiplier`)) _actiontoughnessdamagemultiplier (select `/Game/CombatSystem/Blueprints/Enums/E_AttackType` _attacktypeforhitreflection :`NewEnumerator6` "NewEnumerator3" :`NewEnumerator0` "NewEnumerator0" :`NewEnumerator2` "NewEnumerator1" :`NewEnumerator3` "NewEnumerator2" :`NewEnumerator7` "NewEnumerator4" :`NewEnumerator8` "NewEnumerator5" :`NewEnumerator9` "NewEnumerator6" :`NewEnumerator10` "NewEnumerator7" :`NewEnumerator11` "NewEnumerator8" :!type "/Game/CombatSystem/NPC/Data/E_NPC_DamageType Enum"))
          (`self.K2_SetActorLocation` _hitactor (`KismetMathLibrary.VLerp` (`self.K2_GetActorLocation` _hitactor) (`self.K2_GetActorLocation`) 0.1) false false))))))

(event `self.ReceiveTick`
  (params (DeltaSeconds :type "Float (single-precision)"))
  (bind _arrow (`self.Arrow`))
  (bind _returnvalue (`SceneComponent.K2_GetComponentLocation` _arrow))
  (`SceneComponent.K2_AddWorldRotation` (`self.Cube`) (`KismetMathLibrary.MakeRotator` 0.0 0.0 (* (`self.Speed`) 1.0)) false false)
  (bind (_outhit _returnvalue_2) (`KismetSystemLibrary.LineTraceSingleForObjects` _returnvalue (+ _returnvalue (* (`SceneComponent.GetForwardVector` _arrow) (`KismetMathLibrary.Conv_DoubleToVector` 500.0))) (`|MakeArray` "ObjectTypeQuery1" "ObjectTypeQuery2" :!type "EObjectTypeQuery Enum") false (`|MakeArray` self null :!type "Actor Object Reference") "ForDuration"))
  (if (not _returnvalue_2)
    (`self.K2_AddActorWorldOffset` (* (`SceneComponent.GetForwardVector` (`self.Arrow`)) (`self.Move Speed`)))))

(fn `UserConstructionScript`)