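; Skill component for a combat character that plays montages from a per-skill data map, gated by cooldown components.
; On BeginPlay it waits for the main weapon, then creates a paused looping timer that sphere-traces along the blade to damage NPCs.
; Montage notifies toggle that trace, hide the mesh or spawn slash-wave and tornado actors.
; The dimensional slash (次元斩) repeatedly sets nearby NPCs' status, then deals area damage once its notify ends.
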(event `self.ReceiveBeginPlay`
  (bind _ascharacter (cast `Character` (`self.GetOwner`)))
  (set `self.Use Skills Characher` _ascharacter)
  (bind _asbp_combat_character (cast `/Game/CombatSystem/Blueprints/BP_CombatCharacter` (`self.Use Skills Characher`) :!label _label))
  (bind _returnvalue (`/Game/CombatSystem/Blueprints/Components/BP_CombatComponent.GetMainWeapon` (`/Game/CombatSystem/Blueprints/BP_CombatCharacter.CombatComponent` _asbp_combat_character)))
  (`/Engine/EditorBlueprintResources/StandardMacros.IsValid` _returnvalue
    (:`Is Valid`
      (set `self.Use Weapen Static Mesh` (`/Game/CombatSystem/Blueprints/Actor/Bp_BaseEquippable.ItemStaticMesh` _returnvalue))
      (set `self.武器模型长度` (* (.y (`.BoxExtent` (`KismetSystemLibrary.GetComponentBounds` (`self.Use Weapen Static Mesh`)))) 2.0))
      (bind _returnvalue_2 (`KismetSystemLibrary.K2_SetTimer` null "Attack Determination Function" 0.005 true))
      (bind _output_get (set `self.Attack Determination Timer` _returnvalue_2))
      (`KismetSystemLibrary.K2_PauseTimerHandle` _output_get))
    (:`Is Not Valid`
      (`KismetSystemLibrary.Delay` 0.2)
      (goto _label))))

(event `Use Skill`
  (params (Skills :type "/Game/CombatSystem/Blueprints/SkillBlueprints/E_SkillType Enum" :default "NewEnumerator0"))
  (set `self.Skills Enum` Skills)
  (if (not (`.EnterCooling_31_2B9C6D354898D1603C0BC48BA897C267` (break `/Game/CombatSystem/Blueprints/Structs/F_AttackMoves` (`BlueprintMapLibrary.Map_Find` (`self.Skill Animation Data`) (`self.Skills Enum`)))))
    (`self.Set Characert State` "NewEnumerator1")
    (bind _notifyname (`|PlayMontage` (`Character.Mesh` (`self.Use Skills Characher`)) (`|GetArrayItem` (`.Animation_45_1C6917A044DC51727F0F91935B0E5A51` (break `/Game/CombatSystem/Blueprints/Structs/F_AttackMoves` (`BlueprintMapLibrary.Map_Find` (`self.Skill Animation Data`) (`self.Skills Enum`))))))
      (:`then`
        (`self.Set Whether To Allow Movement` (`.AllowMovement?_29_A5E35928453D1428C38A0697B4C48272` (break `/Game/CombatSystem/Blueprints/Structs/F_AttackMoves` (`BlueprintMapLibrary.Map_Find` (`self.Skill Animation Data`) (`self.Skills Enum`)))))
        (`self.Add Cooling Component`))
      (:`OnCompleted`
        (`self.Set Characert State` "NewEnumerator1")
        (`self.Set Whether To Allow Movement` true))
      (:`OnNotifyBegin`
        (`self.动画通知处理` _notifyname))
      (:`OnNotifyEnd`
        (switch `name` _notifyname
          (:`攻击`
            (`self.Set Stat Or End Attack Determination` false))
          (:`消失`
            (`SceneComponent.SetHiddenInGame` (`Character.Mesh` (`self.Use Skills Characher`)) false true))
          (:`次元斩`
            (set `self.完成次元斩` true)))))))

(event `动画通知处理`
  (params (`Noptify Name` :type Name))
  (bind _returnvalue (`Actor.K2_GetActorLocation` (`self.Use Skills Characher`)))
  (bind (_returnvalue_location _returnvalue_rotation) (`KismetMathLibrary.BreakTransform` (`Actor.GetTransform` (`self.Use Skills Characher`))))
  (bind (_returnvalue_location_2 _returnvalue_rotation_2) (`KismetMathLibrary.BreakTransform` (`Actor.GetTransform` (`self.Use Skills Characher`))))
  (bind _returnvalue_2 (`Actor.K2_GetActorLocation` (`self.Use Skills Characher`)))
  (switch `name` `Noptify Name`
    (:`攻击`
      (`self.Set Stat Or End Attack Determination` true))
    (:`跳斩剑气`
      (`|SpawnActorFromClass` "/Game/CombatSystem/Blueprints/SkillBlueprints/BP_跳斩剑气.BP_跳斩剑气_C" (`KismetMathLibrary.MakeTransform` _returnvalue_location _returnvalue_rotation) "AlwaysSpawn" "MultiplyWithRoot" null (`BlueprintMapLibrary.Map_Find` (`self.Skill Animation Data`) (`self.Skills Enum`)) 2.5 (`self.Use Skills Characher`) null))
    (:`龙卷风摧毁停车场`
      (`|SpawnActorFromClass` "/Game/CombatSystem/Blueprints/SkillBlueprints/BP_龙卷风.BP_龙卷风_C" (`KismetMathLibrary.MakeTransform` _returnvalue_location_2 _returnvalue_rotation_2) "AlwaysSpawn" "MultiplyWithRoot" null (`self.Use Skills Characher`) (`BlueprintMapLibrary.Map_Find` (`self.Skill Animation Data`) (`self.Skills Enum`)) 2.5 null))
    (:`消失`
      (`SceneComponent.SetHiddenInGame` (`Character.Mesh` (`self.Use Skills Characher`)) true true))
    (:`次元斩`
      (bind (_outhits _returnvalue_3) (`KismetSystemLibrary.SphereTraceMultiForObjects` :`Start` _returnvalue_2 :`End` _returnvalue_2 :`Radius` 3000.0 :`ObjectTypes` (`|MakeArray` "ObjectTypeQuery3" :!type "EObjectTypeQuery Enum") :`DrawDebugType` "ForDuration" :!label _label_2))
      (if _returnvalue_3
        (for _array_element _outhits
          (bind _asbp_new_npc_character (cast `/Game/CombatSystem/NPC/BP_NEW_NPC_Character` (`.HitActor` (`GameplayStatics.BreakHitResult` _array_element))))
          (`/Game/CombatSystem/NPC/C_NPC_DataAndBehaviourManagement_Component.Set NPC Staues` (`/Game/CombatSystem/NPC/BP_NEW_NPC_Character.C_NPC_DataAndBehaviourManagement_Component` _asbp_new_npc_character) "NewEnumerator0"))
        (if (`self.完成次元斩`)
          (set `self.完成次元斩` false)
          (bind (_outhits_2 _returnvalue_4) (`KismetSystemLibrary.SphereTraceMultiForObjects` :`Start` _returnvalue :`End` _returnvalue :`Radius` 3000.0 :`ObjectTypes` (`|MakeArray` "ObjectTypeQuery3" :!type "EObjectTypeQuery Enum") :`DrawDebugType` "ForDuration"))
          (if _returnvalue_4
            (for _array_element_2 _outhits_2
              (bind _returnvalue_5 (`Actor.GetComponentByClass` (`.HitActor` (`GameplayStatics.BreakHitResult` _array_element_2)) "/Game/CombatSystem/NPC/C_NPC_DataAndBehaviourManagement_Component.C_NPC_DataAndBehaviourManagement_Component_C"))
              (`/Engine/EditorBlueprintResources/StandardMacros.IsValid` _returnvalue_5
                (:`Is Valid`
                  (message `/Game/CombatSystem/NPC/NPC_Interactive_Interface.Create Damage` _returnvalue_5 400.0 9999.0 "NewEnumerator0")))))
          (else
            (`KismetSystemLibrary.Delay` 0.2)
            (goto _label_2)))))))

(fn `Add Cooling Component`
  (`|AddComponentByClass` (`self.GetOwner`) "/Game/CombatSystem/NPC/C_NPC_AttackCapabilityCondown.C_NPC_AttackCapabilityCondown_C" null "NewEnumerator0" self false (`self.Skills Enum`)))

(fn `Attack Determination Function`
  (bind _use_weapen_static_mesh (`self.Use Weapen Static Mesh`))
  (bind _returnvalue (`SceneComponent.K2_GetComponentLocation` _use_weapen_static_mesh))
  (bind (_animation _nextcomboinput _actiondamagemultiplier _actiontoughnessdamagemultiplier _actionscd `_斩切槽消耗` _actionssuperarmor _attacktypeforhitreflection) (break `/Game/CombatSystem/Blueprints/Structs/F_AttackMoves` (`BlueprintMapLibrary.Map_Find` (`self.Skill Animation Data`) (`self.Skills Enum`))))
  (bind (_outhits _returnvalue_2) (`KismetSystemLibrary.SphereTraceMultiForObjects` _returnvalue (+ _returnvalue (* (`SceneComponent.GetUpVector` _use_weapen_static_mesh) (`self.武器模型长度`))) 10.0 (`|MakeArray` "ObjectTypeQuery3" :!type "EObjectTypeQuery Enum") false (`|MakeArray` (`self.Use Skills Characher`) :!type "Actor Object Reference") "ForDuration"))
  (if _returnvalue_2
    (for _array_element _outhits
      (bind _returnvalue_3 (`Actor.GetComponentByClass` (`.HitActor` (`GameplayStatics.BreakHitResult` _array_element)) "/Game/CombatSystem/NPC/C_NPC_DataAndBehaviourManagement_Component.C_NPC_DataAndBehaviourManagement_Component_C"))
      (`/Engine/EditorBlueprintResources/StandardMacros.IsValid` _returnvalue_3
        (:`Is Valid`
          (message `/Game/CombatSystem/NPC/NPC_Interactive_Interface.Create Damage` _returnvalue_3 _actiondamagemultiplier _actiontoughnessdamagemultiplier (select `/Game/CombatSystem/Blueprints/Enums/E_AttackType` _attacktypeforhitreflection :`NewEnumerator6` "NewEnumerator3" :`NewEnumerator0` "NewEnumerator0" :`NewEnumerator2` "NewEnumerator1" :`NewEnumerator3` "NewEnumerator2" :`NewEnumerator7` "NewEnumerator4" :`NewEnumerator8` "NewEnumerator5" :`NewEnumerator9` "NewEnumerator6" :`NewEnumerator10` "NewEnumerator7" :`NewEnumerator11` "NewEnumerator8" :!type "/Game/CombatSystem/NPC/Data/E_NPC_DamageType Enum")))))))

(fn `Set Characert State`
  (params (NewState :type "/Game/CombatSystem/Blueprints/Enums/E_CharacterState Enum" :default "NewEnumerator0"))
  (bind _asbp_combat_character (cast `/Game/CombatSystem/Blueprints/BP_CombatCharacter` (`self.Use Skills Characher`)))
  (`/Game/CombatSystem/Blueprints/Components/BP_StateManagerComponent.SetState` (`/Game/CombatSystem/Blueprints/BP_CombatCharacter.StateManagerComponent` _asbp_combat_character) NewState))

(fn `Set Stat Or End Attack Determination`
  (params (`Stat?` :type Boolean))
  (bind _attack_determination_timer (`self.Attack Determination Timer`))
  (if `Stat?`
    (`KismetSystemLibrary.K2_UnPauseTimerHandle` _attack_determination_timer)
    (else
      (`KismetSystemLibrary.K2_PauseTimerHandle` _attack_determination_timer))))

(fn `Set Whether To Allow Movement`
  (params (`Allow?` :type Boolean))
  (if `Allow?`
    (`CharacterMovementComponent.SetMovementMode` (`Character.CharacterMovement` (`self.Use Skills Characher`)) "MOVE_Walking" 0)
    (else
      (`CharacterMovementComponent.DisableMovement` (`Character.CharacterMovement` (`self.Use Skills Characher`))))))