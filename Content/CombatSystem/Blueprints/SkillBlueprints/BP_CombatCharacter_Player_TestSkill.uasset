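; Player combat character, apparently a skill test variant, that spawns a katana and adds lock-on targeting, executions, potion healing and a skill/item menu toggle.
; Executions pick the locked or closest low-health victim in range and play a random paired montage.
; The timeline-driven cable grapple pulls locked targets to the player, or pulls the player to traced "CanGrapple" surfaces.
; Damage notifications route through BPCLai's link-time and invincibility checks before toughness-gated hit reactions.
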(event `self.ReceiveBeginPlay`
  (`parent.ReceiveBeginPlay`)
  (bind _returnvalue (`|SpawnActorFromClass` "/Game/CombatSystem/Blueprints/Actor/BP_Katana_Sword.BP_Katana_Sword_C" (`self.GetTransform`) "Undefined" "MultiplyWithRoot" self null))
  (`/Game/CombatSystem/Blueprints/Actor/Bp_BaseEquippable.OnEquipped` _returnvalue)
  (`/Game/CombatSystem/Blueprints/Components/BP_StatsComponent.InitializeStats` (`self.StatsComponent`))
  (`/Game/Lai/BPC_Lai.Init` (`self.BPC_Lai`) self (`self.TargetSystem`) (`self.NS_juhexuli_Buff_Lv2`))
  (bind _aswb_stat_bar (cast `/Game/CombatSystem/UI/WB_StatBar` (`WidgetComponent.GetWidget` (`self.PlayerUI`))))
  (set `self.Stat Bar` (`/Game/CombatSystem/UI/WB_StatBar.StatBar` _aswb_stat_bar))
  (`UserWidget.AddToViewport` _aswb_stat_bar 0)
  (add `/Game/CombatSystem/Blueprints/Components/BP_StatsComponent.OnCurrentStatValueUpdated` (`self.StatsComponent`) (`|CreateDelegate` :!event `OnStatValueUpdated`)))

(event `InputAction|LightAttackInput`
  (params (Key :type "Key Structure"))
  ;[1 1 1] Light Attack with Charge Attack
)

(event `InputAction|TargetEnemy`
  (params (Key :type "Key Structure"))
  ;[1 1 1] Target System
  (:`Pressed`
    (`TargetSystemComponent.TargetActor` (`self.TargetSystem`))))

(event `InputAxis|ChangeTargets`
  (params (AxisValue :type "Float (single-precision)"))
  ;[1 1 1] Target System
  (`TargetSystemComponent.TargetActorWithAxisInput` (`self.TargetSystem`) AxisValue))

(event `self.TargetSystem.OnTargetLockedOn`
  (params (TargetActor :type "Actor Object Reference"))
  ;[1 1 1] Target System
  (set `self.TargetLockOn` TargetActor)
  (set `self.IsLockingTarget` true))

(event `self.TargetSystem.OnTargetLockedOff`
  (params (TargetActor :type "Actor Object Reference"))
  ;[1 1 1] Target System
  (set `self.TargetLockOn` null)
  (set `self.IsLockingTarget` false))

(event `InputAction|Execution`
  (params (Key :type "Key Structure"))
  ;[1 0 0.02238] Execution System (Attacker)
  (:`Pressed`
    (set `self.Victim` null)
    (`KismetArrayLibrary.Array_Clear` (`self.CanExeuctionTargets`))
    (if (`self.IsLockingTarget`)
      (`/Engine/EditorBlueprintResources/StandardMacros.IsValid` (`self.TargetLockOn`)
        (:`Is Valid`
          (bind _asbp_combat_character (cast `/Game/CombatSystem/Blueprints/BP_CombatCharacter` (`self.TargetLockOn`)))
          (`/Engine/EditorBlueprintResources/StandardMacros.IsValid` _asbp_combat_character
            (:`Is Valid`
              (if (and (<= (`/Game/CombatSystem/Blueprints/Components/BP_StatsComponent.GetPercentStatValue` (`/Game/CombatSystem/Blueprints/BP_CombatCharacter.StatsComponent` _asbp_combat_character) "NewEnumerator1") (`self.CanExeuctionHealthPercent`)) (<= (`self.GetDistanceTo` (`self.TargetLockOn`) self) (`self.Excution Distance`)))
                (set `self.Victim` (`self.TargetLockOn`))
                (`self.CS_PerformExeucting`))))))
      (else
        (bind _outactors (`KismetSystemLibrary.SphereOverlapActors` (`self.K2_GetActorLocation`) (`self.Excution Distance`) (`|MakeArray` "ObjectTypeQuery3" :!type "EObjectTypeQuery Enum") null (`|MakeArray` self :!type "Actor Object Reference")))
        (for _array_element _outactors
          (bind _asbp_combat_character_2 (cast `/Game/CombatSystem/Blueprints/BP_CombatCharacter` _array_element))
          (`/Engine/EditorBlueprintResources/StandardMacros.IsValid` _asbp_combat_character_2
            (:`Is Valid`
              (if (<= (`/Game/CombatSystem/Blueprints/Components/BP_StatsComponent.GetPercentStatValue` (`/Game/CombatSystem/Blueprints/BP_CombatCharacter.StatsComponent` _asbp_combat_character_2) "NewEnumerator0") (`self.CanExeuctionHealthPercent`))
                (`KismetArrayLibrary.Array_Add` (`self.CanExeuctionTargets`) _asbp_combat_character_2)))))
        (for _array_element_2 (`self.CanExeuctionTargets`)
          (bind _returnvalue (`self.GetDistanceTo` _array_element_2 self))
          (if (< _returnvalue (`self.ClosestDistance`))
            (set `self.ClosestDistance` _returnvalue)
            (set `self.Victim` _array_element_2)))
        (`/Engine/EditorBlueprintResources/StandardMacros.IsValid` (`self.Victim`)
          (:`Is Valid`
            (set `self.ClosestDistance` 9999.0)
            (`self.CS_PerformExeucting`)))))))

(event `InputAction|Grapple`
  (params (Key :type "Key Structure"))
  (bind _followcamera (`self.FollowCamera`))
  (bind _returnvalue (`SceneComponent.K2_GetComponentLocation` _followcamera))
  (bind _returnvalue_2 (`SceneComponent.K2_GetComponentLocation` (`Actor.RootComponent` (`self.TargetLockOn`))))
  (bind (_returnvalue_roll _returnvalue_pitch _returnvalue_yaw) (`KismetMathLibrary.BreakRotator` (`KismetMathLibrary.FindLookAtRotation` (`self.K2_GetActorLocation`) (`SceneComponent.K2_GetComponentLocation` (`Actor.RootComponent` (`self.TargetLockOn`))))))
  (bind _returnvalue_3 (+ (`SceneComponent.K2_GetComponentLocation` (`self.Cable`)) (* (`KismetMathLibrary.GetForwardVector` (`SceneComponent.K2_GetComponentRotation` (`self.FollowCamera`))) (`self.GrappleLongest`))))
  ;[1 0 0.01661] Grapple
  (:`Pressed`
    ;;[1 1 1] 创建钩爪的射线
    (if (not (`self.IsGraping`))
      (set `self.IsGraping` true)
      (set `self.AttackTypeForHitReflection` "NewEnumerator3")
      (`SceneComponent.SetVisibility` (`self.Cable`) true false)
      (set `self.ForwardVector` (`SceneComponent.GetForwardVector` (`self.FollowCamera`)))
      (if (`self.IsLockingTarget`)
        ;;[1 1 1] 锁定敌人的时候的钩爪逻辑
        (`self.K2_SetActorRotation` (`KismetMathLibrary.MakeRotator` 0.0 0.0 _returnvalue_yaw))
        (bind (_direction _alpha) (`Timeline|Timeline_6` :!via `PlayFromStart`)
          (:`Update`
            (`SceneComponent.K2_SetWorldLocation` (`self.TmpMesh`) (`KismetMathLibrary.VLerp` (`SceneComponent.K2_GetComponentLocation` (`self.Cable`)) _returnvalue_2 _alpha) false false))
          (:`Finished`
            (`|ExecutionSequence`
              (:`then_0`
                (bind (_direction_2 _alpha_2) (`Timeline|Timeline_7` :!via `ReverseFromEnd`)
                  (:`Update`
                    (`SceneComponent.K2_SetWorldLocation` (`self.TmpMesh`) (`KismetMathLibrary.VLerp` (`SceneComponent.K2_GetComponentLocation` (`self.Cable`)) _returnvalue_2 _alpha_2) false false))))
              (:`then_1`
                (bind _output_get (set `self.PlayerLocation` (`self.K2_GetActorLocation`)))
                (bind _asbp_new_npc_character (cast `/Game/CombatSystem/NPC/BP_NEW_NPC_Character` (`self.TargetLockOn`)))
                (`/Game/CombatSystem/NPC/C_NPC_DataAndBehaviourManagement_Component.Create Damage` (`/Game/CombatSystem/NPC/BP_NEW_NPC_Character.C_NPC_DataAndBehaviourManagement_Component` _asbp_new_npc_character) 0.0 0.0 "NewEnumerator2")
                (bind (_direction_3 _alpha_3) (`Timeline|Timeline_8`)
                  (:`Update`
                    (`self.K2_SetActorLocation` (`self.TargetLockOn`) (`KismetMathLibrary.VLerp` (`SceneComponent.K2_GetComponentLocation` (`Actor.RootComponent` (`self.TargetLockOn`))) (`KismetMathLibrary.MakeVector` (.x _output_get) (.y _output_get) (+ (.z _output_get) 100.0)) _alpha_3) true false))
                  (:`Finished`
                    (set `self.IsGraping` false)
                    (`SceneComponent.SetVisibility` (`self.Cable`) false false)
                    (set `self.AttackTypeForHitReflection` "NewEnumerator6")))))))
        (else
          (bind (_outhit _returnvalue_4) (`KismetSystemLibrary.LineTraceSingle` :`Start` _returnvalue :`End` (+ _returnvalue (* (`KismetMathLibrary.GetForwardVector` (`SceneComponent.K2_GetComponentRotation` _followcamera)) (`self.GrappleLongest`))) :`TraceChannel` "TraceTypeQuery1" :`DrawDebugType` "ForDuration"))
          (`self.Character facing camera`)
          (if _returnvalue_4
            (if (`self.ActorHasTag` (`.HitActor` (`GameplayStatics.BreakHitResult` _outhit)) "CanGrapple")
              (bind (_direction_4 _alpha_4) (`Timeline|Timeline_3` :!via `PlayFromStart`)
                (:`Update`
                  (`SceneComponent.K2_SetWorldLocation` (`self.TmpMesh`) (`KismetMathLibrary.VLerp` (`SceneComponent.K2_GetComponentLocation` (`self.Cable`)) (`.Location` (`GameplayStatics.BreakHitResult` _outhit)) _alpha_4) false false))
                (:`Finished`
                  (`|ExecutionSequence`
                    (:`then_0`
                      (bind (_direction_5 _alpha_5) (`Timeline|Timeline_4` :!via `ReverseFromEnd`)
                        (:`Update`
                          (`SceneComponent.K2_SetWorldLocation` (`self.TmpMesh`) (`KismetMathLibrary.VLerp` (`SceneComponent.K2_GetComponentLocation` (`self.Cable`)) (`.Location` (`GameplayStatics.BreakHitResult` _outhit)) _alpha_5) false false))))
                    (:`then_1`
                      ;;[1 1 1] 先获取玩家当前位置，然后使用timeline和lerp来让来判断玩家和钩爪终点的相对位置并移动过去
                      (bind _output_get_2 (set `self.PlayerLocation` (`self.K2_GetActorLocation`)))
                      (bind (_direction_6 _alpha_6) (`Timeline|Timeline_5` :!via `PlayFromStart`)
                        (:`Update`
                          (`self.K2_SetActorLocation` (`KismetMathLibrary.VLerp` _output_get_2 (`KismetMathLibrary.MakeVector` (.x (`.Location` (`GameplayStatics.BreakHitResult` _outhit))) (.y (`.Location` (`GameplayStatics.BreakHitResult` _outhit))) (+ (.z (`.Location` (`GameplayStatics.BreakHitResult` _outhit))) 200.0)) _alpha_6) true))
                        (:`Finished`
                          (`self.LaunchCharacter` (* (`self.ForwardVector`) 200.0) true true)
                          (set `self.IsGraping` false)
                          (`SceneComponent.SetVisibility` (`self.Cable`) false false)
                          (set `self.AttackTypeForHitReflection` "NewEnumerator6")))))))
              (else
                (bind (_direction_7 _alpha_7) (`Timeline|Timeline_1` :!via `PlayFromStart`)
                  (:`Update`
                    (`SceneComponent.K2_SetWorldLocation` (`self.TmpMesh`) (`KismetMathLibrary.VLerp` (`SceneComponent.K2_GetComponentLocation` (`self.Cable`)) (`.Location` (`GameplayStatics.BreakHitResult` _outhit)) _alpha_7) false false))
                  (:`Finished`
                    (bind (_direction_8 _alpha_8) (`Timeline|Timeline_2` :!via `ReverseFromEnd`)
                      (:`Update`
                        (`SceneComponent.K2_SetWorldLocation` (`self.TmpMesh`) (`KismetMathLibrary.VLerp` (`SceneComponent.K2_GetComponentLocation` (`self.Cable`)) (`.Location` (`GameplayStatics.BreakHitResult` _outhit)) _alpha_8) false false))
                      (:`Finished`
                        (set `self.IsGraping` false :!label _label)
                        (`SceneComponent.SetVisibility` (`self.Cable`) false false)
                        (set `self.AttackTypeForHitReflection` "NewEnumerator6")))))))
            (else
              ;;[1 1 1] 根据射线长度生成钩爪长度
              (bind (_direction_9 _alpha_9) (`Timeline|Timeline` :!via `PlayFromStart`)
                (:`Update`
                  (`SceneComponent.K2_SetWorldLocation` (`self.TmpMesh`) (`KismetMathLibrary.VLerp` (`SceneComponent.K2_GetComponentLocation` (`self.Cable`)) _returnvalue_3 _alpha_9) false false))
                (:`Finished`
                  (bind (_direction_10 _alpha_10) (`Timeline|Timeline_0` :!via `ReverseFromEnd`)
                    (:`Update`
                      (`SceneComponent.K2_SetWorldLocation` (`self.TmpMesh`) (`KismetMathLibrary.VLerp` (`SceneComponent.K2_GetComponentLocation` (`self.Cable`)) _returnvalue_3 _alpha_10) false false))
                    (:`Finished`
                      (goto _label))))))))))))

(event `CS_PerformExeucting`
  (bind _executionmoves (`self.ExecutionMoves`))
  (bind _output_execution_montage (break `/Game/CombatSystem/Blueprints/Structs/F_ExecutionMoves` (`|GetArrayItem` _executionmoves (`self.ExecutionIndex`))))
  ;[1 0 0.02238] Execution System (Attacker)
  (`/Game/CombatSystem/Blueprints/Components/BP_StateManagerComponent.SetState` (`self.StateManagerComponent`) "NewEnumerator10")
  (set `self.ExecutionIndex` (`KismetMathLibrary.RandomInteger` (- (`KismetArrayLibrary.Array_Length` _executionmoves) 1)))
  (`self.SetLocation`)
  (`|PlayMontage` (`self.Mesh`) _output_execution_montage
    (:`then`
      (message `/Game/CombatSystem/Blueprints/Interface/ExecutionBPI.PlayVictimMontage` (`self.Victim`) (`self.ExecutionIndex`) self))))

(event `self.StatsComponent.受到伤害通知`
  (params (Actro :type "Actor Object Reference") (`是否打断?` :type Boolean))
  (bind (_returnvalue_roll _returnvalue_pitch _returnvalue_yaw) (`KismetMathLibrary.BreakRotator` (`KismetMathLibrary.FindLookAtRotation` (`self.K2_GetActorLocation`) (`self.K2_GetActorLocation` Actro))))
  ;[1 0.06442 0] Damage
  (if (`/Game/Lai/BPC_Lai.CanIntoLinkTime` (`self.BPC_Lai`))
    (set `/Game/Lai/BPC_Lai.ShoundIntoLinkTime` true (`self.BPC_Lai`))
    (elif (not (`/Game/Lai/BPC_Lai.Invincent` (`self.BPC_Lai`)))
      (set `/Game/Lai/BPC_Lai.LaiHold` false (`self.BPC_Lai`))
      (set `/Game/Lai/BPC_Lai.CanLai` false (`self.BPC_Lai`))
      (set `/Game/Lai/BPC_Lai.CurrentHoldTime` 0.0 (`self.BPC_Lai`))
      (`/Engine/EditorBlueprintResources/StandardMacros.IsValid` Actro
        (:`Is Valid`
          ;;[1 1 1] 音效
          (`GameplayStatics.PlaySoundAtLocation` "/Game/CombatSystem/Dialogues/CG1_SFX/SFX_Sources/CG1_Silence.CG1_Silence" (`self.K2_GetActorLocation` Actro) (struct) 1.0 1.0 0.0 null null null null)
          (if (`self.ActorHasTag` Actro "NPC")
            ;;[1 1 1] 让受击者朝向朝着攻击者的位置
            (`self.K2_SetActorRelativeRotation` Actro (`KismetMathLibrary.MakeRotator` 0.0 0.0 _returnvalue_yaw) false false)))
        (:`Is Not Valid`
          _))
      ;;[1 1 1] 受击特效
      (`GameplayStatics.SpawnEmitterAtLocation` null (`self.K2_GetActorLocation`) (struct) (0.7 0.7 0.7))
      (if (`self.CanReceieveHitReaction?`)
        ;;[1 1 1] 韧性判定，若不为0则不执行受击动画
        (if (<= (`/Game/CombatSystem/Blueprints/Components/BP_StatsComponent.GetCurrentStatValue` (`self.StatsComponent`) "NewEnumerator5") 0.0)
          (`/Game/CombatSystem/Blueprints/Components/BP_StateManagerComponent.SetState` (`self.StateManagerComponent`) "NewEnumerator5")
          (if `是否打断?`
            (`self.PlayAnimMontage` "/Game/Katana_Animations/NEWanim/08_Hit/02_Hit_Combat/03_Hit_Combat_Large/AS_Hit_Combat_Large_F_Seq_Montage.AS_Hit_Combat_Large_F_Seq_Montage")
            (`/Game/CombatSystem/Blueprints/Components/BP_StateManagerComponent.SetState` (`self.StateManagerComponent`) "NewEnumerator0")
            (else
              (`/Game/CombatSystem/Blueprints/Components/BP_StateManagerComponent.SetState` (`self.StateManagerComponent`) "NewEnumerator0"))))))))

(event `self.ResetCombat`
  (`parent.ResetCombat`))

(event `self.ResetAttack`
  (`parent.ResetAttack`))

(event `ToggleCanLaiEffect`
  (params (bNewVisibility :type Boolean))
  (`SceneComponent.SetVisibility` (`self.NS_juhexuli_Buff_Lv2`) bNewVisibility false))

(event `Key|One`
  (params (Key :type "Key Structure"))
  (:`Pressed`
    (`/Game/CombatSystem/Blueprints/SkillBlueprints/C_SkillComponent.Use Skill` (`self.C_SkillComponent`) "NewEnumerator5")))

(event `OnStatValueUpdated`
  (params (StatType :type "/Game/CombatSystem/Blueprints/Enums/E_Stats Enum" :default "NewEnumerator0") (Value :type "Float (double-precision)"))
  (if (`|EnumEquality` StatType (`self.StatType`))
    (bind _statscomponent (`self.StatsComponent`)
      (:`then`
        (`ProgressBar.SetPercent` (`self.Stat Bar`) (/ Value (`/Game/CombatSystem/Blueprints/Components/BP_StatsComponent.GetMaxStatValue` _statscomponent (`self.StatType`)))))
      (:`else`))))

(event `InputAction|Use health potion`
  (params (Key :type "Key Structure"))
  (bind _health_potion_restore (`self.Health potion restore`))
  ;[1 1 1] 使用药瓶回血
  (:`Pressed`
    (if (>= (`self.Health_potion`) 1)
      (set `self.Health_potion` (- (`self.Health_potion`) 1))
      (`/Game/CombatSystem/Blueprints/Components/BP_StatsComponent.SetCurrentStatValue` (`self.StatsComponent`) "NewEnumerator1" (`KismetMathLibrary.FClamp` (+ (`/Game/CombatSystem/Blueprints/Components/BP_StatsComponent.GetCurrentStatValue` (`self.StatsComponent`) "NewEnumerator1") _health_potion_restore) _health_potion_restore (`/Game/CombatSystem/Blueprints/Components/BP_StatsComponent.GetMaxStatValue` (`self.StatsComponent`) "NewEnumerator1"))))))

(event `InputAction|Toggle Menu`
  (params (Key :type "Key Structure"))
  ;[1 1 1] 按Tab切换道具和技能栏
  (:`Pressed`
    (if (`self.Is Menu Open`)
      (`/Engine/EditorBlueprintResources/StandardMacros.IsValid` (`self.Skill Menu widget`)
        (:`Is Valid`
          (`Widget.RemoveFromParent` (`self.Skill Menu widget`))
          (set `self.Is Menu Open` true)
          (`KismetSystemLibrary.Delay` 0.2)
          (`UserWidget.AddToViewport` (`self.Item Menu widget`) 0)
          (set `self.Is Menu Open` false)))
      (else
        (`/Engine/EditorBlueprintResources/StandardMacros.IsValid` (`self.Item Menu widget`)
          (:`Is Valid`
            (`Widget.RemoveFromParent` (`self.Item Menu widget`))
            (set `self.Is Menu Open` false)
            (`KismetSystemLibrary.Delay` 0.2)
            (`UserWidget.AddToViewport` (`self.Skill Menu widget`) 0)
            (set `self.Is Menu Open` true)))))))

(event `self.BeginPlay`
  ;[1 1 1] 开始时技能栏显示
  (`UserWidget.AddToViewport` (`self.Skill Menu widget`) 0)
  (set `self.Is Menu Open` true))

(fn `Character facing camera`
  (bind _returnvalue (`self.K2_GetActorLocation`))
  (bind (_returnvalue_roll _returnvalue_pitch _returnvalue_yaw) (`KismetMathLibrary.BreakRotator` (`KismetMathLibrary.FindLookAtRotation` _returnvalue (+ (`SceneComponent.GetForwardVector` (`self.FollowCamera`)) _returnvalue))))
  (`self.K2_SetActorRotation` (`KismetMathLibrary.MakeRotator` 0.0 0.0 _returnvalue_yaw)))

(fn `IsTargetable`
  (returns (ReturnValue :type Boolean))
  (return false))

(fn `UserConstructionScript`
  (`parent.UserConstructionScript`))