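; Jump-slash sword energy projectile (跳斩剑气) that damages the first NPC it hits, then destroys itself.
; Each Tick it moves along its arrow by Speed, unscaled by delta time, then sphere-traces between two marker components, ignoring itself and its releaser, with debug drawing on.
; Hits on actors with the NPC data/behaviour component send a damage message built from AttackMoesData, including scaled damage, toughness damage and mapped hit-reaction type.
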(event `self.ReceiveTick`
  (params (DeltaSeconds :type "Float (single-precision)"))
  (bind (_animation _actiondamagemultiplier _actiontoughnessdamagemultiplier _actionscd `_斩切槽消耗` _actionssuperarmor _attacktypeforhitreflection) (break `/Game/CombatSystem/Blueprints/Structs/F_AttackMoves` (`self.Attack Moes Data`)))
  (`self.K2_AddActorWorldOffset` (* (`SceneComponent.GetForwardVector` (`self.Arrow`)) (`self.Speed`)))
  (bind (_outhit _returnvalue) (`KismetSystemLibrary.SphereTraceSingleForObjects` (`SceneComponent.K2_GetComponentLocation` (`self.State Location`)) (`SceneComponent.K2_GetComponentLocation` (`self.End Location`)) 0.0 (`|MakeArray` "ObjectTypeQuery1" "ObjectTypeQuery2" "ObjectTypeQuery3" "ObjectTypeQuery4" "ObjectTypeQuery5" "ObjectTypeQuery6" "ObjectTypeQuery7" :!type "EObjectTypeQuery Enum") false (`|MakeArray` self (`self.Releases Actor`) :!type "Actor Object Reference") "ForDuration"))
  (if _returnvalue
    (bind _returnvalue_2 (`self.GetComponentByClass` (`.HitActor` (`GameplayStatics.BreakHitResult` _outhit)) "/Game/CombatSystem/NPC/C_NPC_DataAndBehaviourManagement_Component.C_NPC_DataAndBehaviourManagement_Component_C"))
    (`/Engine/EditorBlueprintResources/StandardMacros.IsValid` _returnvalue_2
      (:`Is Valid`
        (message `/Game/CombatSystem/NPC/NPC_Interactive_Interface.Create Damage` _returnvalue_2 (* _actiondamagemultiplier (`self.Damage Multiplier`)) _actiontoughnessdamagemultiplier (select `/Game/CombatSystem/Blueprints/Enums/E_AttackType` _attacktypeforhitreflection :`NewEnumerator6` "NewEnumerator3" :`NewEnumerator0` "NewEnumerator0" :`NewEnumerator2` "NewEnumerator1" :`NewEnumerator3` "NewEnumerator2" :`NewEnumerator7` "NewEnumerator4" :`NewEnumerator8` "NewEnumerator5" :`NewEnumerator9` "NewEnumerator6" :`NewEnumerator10` "NewEnumerator7" :`NewEnumerator11` "NewEnumerator8" :!type "/Game/CombatSystem/NPC/Data/E_NPC_DamageType Enum"))
        (`self.K2_DestroyActor`)))))

(fn `UserConstructionScript`)