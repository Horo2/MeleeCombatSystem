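; BP_CombatCharacter_Child is a combat character Blueprint that adds enemy lock-on through a TargetSystem component.
; The TargetEnemy input calls TargetActor on the component, whose lock-on and lock-off events update the TargetLockOn reference and IsLockingTarget flag.
; IsTargetable always returns false, marking this character as not targetable.
; BeginPlay, overlap and Tick are disabled placeholder nodes, and construction only calls the parent.
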(event `InputAction|TargetEnemy`
  (params (Key :type "Key Structure"))
  ;[1 1 1] Target System
  (:`Pressed`
    (`TargetSystemComponent.TargetActor` (`self.TargetSystem`))))

(event `self.TargetSystem.OnTargetLockedOn`
  (params (TargetActor :type "Actor Object Reference"))
  ;[1 1 1] Target System
  (set `self.TargetLockOn` TargetActor)
  (set `self.IsLockingTarget` true))

(event `self.TargetSystem.OnTargetLockedOff`
  (params (TargetActor :type "Actor Object Reference"))
  ;[1 1 1] Target System
  (set `self.TargetLockOn` null)
  (set `self.IsLockingTarget` false))

(fn `IsTargetable`
  (returns (ReturnValue :type Boolean))
  (return false))

(fn `UserConstructionScript`
  (`parent.UserConstructionScript`))