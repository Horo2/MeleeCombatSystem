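; Anim notify state that opens a combo window during attack animations on BP_CombatCharacter.
; Each tick it enables next-attack input buffering and sends the saved input type through the ContinueNextComboAttack message to chain the combo.
; When the window ends, it disables buffering and resets the saved input to the enum's first entry, clearing the cache.
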(fn `Received_NotifyEnd`
  (params (MeshComp :type "SkeletalMeshComponent Object Reference") (Animation :type "AnimSequenceBase Object Reference") (EventReference :type "AnimNotifyEventReference Structure (by ref)"))
  (returns (ReturnValue :type Boolean))
  (bind _asbp_combat_character (cast `/Game/CombatSystem/Blueprints/BP_CombatCharacter` (`ActorComponent.GetOwner` MeshComp)))
  ;[1 1 1] 重置可连击窗口，并且清空按键缓存
  (set `/Game/CombatSystem/Blueprints/BP_CombatCharacter.CanSaveNextAttackInput` false _asbp_combat_character)
  (set `/Game/CombatSystem/Blueprints/BP_CombatCharacter.SaveInputType` "NewEnumerator0" _asbp_combat_character)
  (return false))

(fn `Received_NotifyTick`
  (params (MeshComp :type "SkeletalMeshComponent Object Reference") (Animation :type "AnimSequenceBase Object Reference") (FrameDeltaTime :type "Float (single-precision)") (EventReference :type "AnimNotifyEventReference Structure (by ref)"))
  (returns (ReturnValue :type Boolean))
  (bind _returnvalue (`ActorComponent.GetOwner` MeshComp))
  (bind _asbp_combat_character (cast `/Game/CombatSystem/Blueprints/BP_CombatCharacter` _returnvalue))
  (set `/Game/CombatSystem/Blueprints/BP_CombatCharacter.CanSaveNextAttackInput` true _asbp_combat_character)
  (message `/Game/CombatSystem/Blueprints/Interface/CombatBPI.ContinueNextComboAttack` _returnvalue (`/Game/CombatSystem/Blueprints/BP_CombatCharacter.SaveInputType` _asbp_combat_character))
  (return false))