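; Melee Zaibatsu soldier AI character Blueprint that implements the NPC's montage-driven attack on top of its parent class.
; A DoOnce gate starts the attack montage; when it completes or is interrupted, a weighted random roll either replays it after a short delay or ends the attack.
; Ending resets the gate, calls the attack completion event and starts the normal-attack cooldown.
; The damage determination notify only prints a debug message.
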(event `self.ReceiveBeginPlay`
  (`parent.ReceiveBeginPlay`))

(event `/Game/CombatSystem/AI/NPCData/NPC_Interface.Attack`
  (`/Engine/EditorBlueprintResources/StandardMacros.DoOnce` false :!label _label
    (:`Completed`
      (set `self.Attacking` true)
      (bind _notifyname (`|PlayMontage` (`self.Mesh`) "/Game/CombatSystem/AI/MeleeZaibatsuSoldier/Animation/INP_Attack_Montage.INP_Attack_Montage" :!label _label_2)
        (:`OnCompleted`
          (if (`KismetMathLibrary.RandomBoolWithWeight` 0.7) :!label _label_3
            (`self.Reset Attack`)
            (`self.Attack Completion Event`)
            (`/Game/CombatSystem/AI/Component/NPC_CoolingComponents.激活普通攻击冷却` (`self.NPC_CoolingComponents`))
            (else
              (`KismetSystemLibrary.Delay` 0.2)
              (goto _label_2))))
        (:`OnInterrupted`
          (goto _label_3))
        (:`OnNotifyBegin`
          (switch `name` _notifyname
            (:`Damage Determination`
              (`KismetSystemLibrary.PrintString` "NPC:开始伤害判定" true true (struct :`R` 1.0 :`G` 0.068885 :`A` 1.0) 0.1))))))))

(event `Reset Attack`
  (goto _label :!via `Reset`))

(fn `UserConstructionScript`
  (`parent.UserConstructionScript`))