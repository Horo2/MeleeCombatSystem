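; AI controller for combat NPCs that runs the remote behavior tree for BP_Ai_Character_Remote pawns and the melee tree otherwise.
; Each tick, a forward sphere trace makes a moving, grounded NPC jump obstacles, with an upward offset nudge.
; Detour and grenade cooldowns each spawn a temporary cooling component that restores an availability flag on completion.
; GetDesireAttack picks between two attack-desire values by whether the given pawn projects inside the player's viewport.
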(event `self.ReceiveBeginPlay`)

(event `self.ReceivePossess`
  (params (PossessedPawn :type "Pawn Object Reference"))
  (set `self.NPC` (cast `Character` PossessedPawn :!pure true))
  (`self.RunBehaviorTree` (select `bool` (`.bSuccess` (cast `/Game/CombatSystem/AI/BP/Remote/BP_Ai_Character_Remote` (`self.NPC`) :!pure true)) :`false` "/Game/CombatSystem/AI/BehaviorTree/Melee/BT_MeleeBehaviorTree.BT_MeleeBehaviorTree" :`true` "/Game/CombatSystem/AI/BehaviorTree/Remotely/BT_RemotelyBehaciorTree.BT_RemotelyBehaciorTree" :!type "BehaviorTree Object Reference")))

(event `self.ReceiveTick`
  (params (DeltaSeconds :type "Float (single-precision)"))
  (bind _npc (`self.NPC`))
  (bind _npc_2 (`self.NPC`))
  (bind _returnvalue (`self.K2_GetActorLocation` _npc_2))
  ;[1 1 1] 跳跃判断
  (if (`NavMovementComponent.IsFalling` (`Character.CharacterMovement` (`self.NPC`)))
    _
    (elif (>= (`KismetMathLibrary.VSize` (`self.GetVelocity` (`self.NPC`))) 100.0)
      (bind (_outhit _returnvalue_2) (`KismetSystemLibrary.SphereTraceSingle` _returnvalue (+ _returnvalue (* (`self.GetActorForwardVector` _npc_2) (`self.Jump Detection Distance`))) 20.0 "TraceTypeQuery1"))
      (if _returnvalue_2
        (`Character.Jump` _npc)
        (`self.K2_AddActorLocalOffset` _npc (0.0 0.0 50.0) false false)))))

(event `激活迂回冷却`
  (params (`Time Required For Cooling` :type "Float (double-precision)"))
  ;[1 1 1] 迂回冷却
  (`/Engine/EditorBlueprintResources/StandardMacros.IsValid` (`self.Detour Cooling Components`)
    (:`Is Not Valid`
      (set `self.Whether Detouring Is Possible?` false)
      (bind _returnvalue (`|AddComponentByClass` "/Game/CombatSystem/AI/BP/CoolingCalculationComponents.CoolingCalculationComponents_C" `Time Required For Cooling`))
      (set `self.Detour Cooling Components` _returnvalue)
      (add `/Game/CombatSystem/AI/BP/CoolingCalculationComponents.Cooling Complete Event` (`self.Detour Cooling Components`) (delegate `Derouring Cooling Complete Event`)))))

(event `Derouring Cooling Complete Event`
  ;[1 1 1] 迂回冷却
  (clear `/Game/CombatSystem/AI/BP/CoolingCalculationComponents.Cooling Complete Event` (`self.Detour Cooling Components`))
  (set `self.Whether Detouring Is Possible?` true)
  (`ActorComponent.K2_DestroyComponent` (`self.Detour Cooling Components`))
  (set `self.Detour Cooling Components` null))

(event `激活手雷冷却`
  (params (`Time Required For Cooling` :type "Float (double-precision)"))
  ;[1 1 1] 手雷冷却
  (`/Engine/EditorBlueprintResources/StandardMacros.IsValid` (`self.Grenade Cooling Components`)
    (:`Is Not Valid`
      (set `self.Grenade` false)
      (bind _returnvalue (`|AddComponentByClass` "/Game/CombatSystem/AI/BP/CoolingCalculationComponents.CoolingCalculationComponents_C" `Time Required For Cooling`))
      (set `self.Grenade Cooling Components` _returnvalue)
      (add `/Game/CombatSystem/AI/BP/CoolingCalculationComponents.Cooling Complete Event` (`self.Grenade Cooling Components`) (delegate `Grenade Cooling Complete Event`)))))

(event `Grenade Cooling Complete Event`
  ;[1 1 1] 手雷冷却
  (clear `/Game/CombatSystem/AI/BP/CoolingCalculationComponents.Cooling Complete Event` (`self.Grenade Cooling Components`))
  (set `self.Grenade` true)
  (`ActorComponent.K2_DestroyComponent` (`self.Grenade Cooling Components`))
  (set `self.Grenade Cooling Components` null))

(fn `Get Desire Attack`
  (params (`Tagt Pawn` :type "Actor Object Reference") (`Within Sight Desire Attack` :type "Float (double-precision)") (`Not Within Sight Desire Attack` :type "Float (double-precision)"))
  (returns (`Desire Attack` :type "Float (double-precision)"))
  (bind (_returnvalue_x _returnvalue_y) (`KismetMathLibrary.BreakVector2D` (`WidgetLayoutLibrary.GetViewportSize`)))
  (bind _screenlocation (`PlayerController.ProjectWorldLocationToScreen` (`GameplayStatics.GetPlayerController` 0) (`self.K2_GetActorLocation` `Tagt Pawn`) false))
  (if (not (or (> (`KismetMathLibrary.BreakVector2D` _screenlocation) _returnvalue_x) (> (`.Y` (`KismetMathLibrary.BreakVector2D` _screenlocation)) _returnvalue_y) (< (`KismetMathLibrary.BreakVector2D` _screenlocation) 0.0) (< (`.Y` (`KismetMathLibrary.BreakVector2D` _screenlocation)) 0.0)))
    (return `Within Sight Desire Attack`)
    (else
      (return `Not Within Sight Desire Attack`))))

(fn `UserConstructionScript`)