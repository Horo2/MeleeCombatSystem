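; BP_JumpingCurve is a helper actor that moves a referenced actor along a jump arc between path points, then destroys itself.
; On BeginPlay it builds a Bezier curve in its local XZ plane from the first and third points, with the midpoint raised by their distance.
; The curve fills a spline, which a timeline samples to set the actor's location.
; When the timeline finishes, it waits briefly and calls a completion event.
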(event `self.ReceiveBeginPlay`
  (bind (_returnvalue_x _returnvalue_y _returnvalue_z) (`KismetMathLibrary.BreakVector` (`KismetMathLibrary.InverseTransformLocation` (`self.GetTransform`) (`|GetArrayItem` (`self.Path Points`) 2))))
  (bind (_returnvalue_x_2 _returnvalue_y_2 _returnvalue_z_2) (`KismetMathLibrary.BreakVector` (`KismetMathLibrary.InverseTransformLocation` (`self.GetTransform`) (`|GetArrayItem` (`self.Path Points`)))))
  (bind _returnvalue (`KismetMathLibrary.InverseTransformLocation` (`self.GetTransform`) (`|GetArrayItem` (`self.Path Points`))))
  (bind _returnvalue_2 (`KismetMathLibrary.InverseTransformLocation` (`self.GetTransform`) (`|GetArrayItem` (`self.Path Points`) 2)))
  (bind (_returnvalue_x_3 _returnvalue_y_3 _returnvalue_z_3) (`KismetMathLibrary.BreakVector` (/ (+ _returnvalue _returnvalue_2) (`KismetStringLibrary.Conv_StringToDouble` "2"))))
  (if (> (`KismetArrayLibrary.Array_Length` (`self.Path Points`)) 2)
    (`KismetArrayLibrary.Array_Clear` (`self.Src`))
    (`KismetArrayLibrary.Array_Add` (`self.Src`) (`KismetMathLibrary.MakeVector2D` _returnvalue_x_2 _returnvalue_z_2))
    (`KismetArrayLibrary.Array_Add` (`self.Src`) (`KismetMathLibrary.MakeVector2D` _returnvalue_x_3 (+ _returnvalue_z_3 (`KismetMathLibrary.Vector_Distance` _returnvalue _returnvalue_2))))
    (`KismetArrayLibrary.Array_Add` (`self.Src`) (`KismetMathLibrary.MakeVector2D` _returnvalue_x (+ _returnvalue_z 90.0)))
    (`SplineComponent.ClearSplinePoints` (`self.Spline`) true)
    (bind _returnvalue_3 (`BerzierCurveComponent.BerzierCurve` (`self.BerzierCurve`) (`self.Src`)))
    (for _array_element _returnvalue_3
      (`SplineComponent.AddSplinePoint` (`self.Spline`) (`KismetMathLibrary.MakeVector` (`KismetMathLibrary.BreakVector2D` _array_element) 0.0 (`.Y` (`KismetMathLibrary.BreakVector2D` _array_element))) "Local" false))
    (`SplineComponent.UpdateSpline` (`self.Spline`))
    (bind (_direction `_新建轨道_0`) (`Timeline|时间轴` :!via `PlayFromStart`)
      (:`Update`
        (`self.K2_SetActorLocation` (`self.Actor`) (`SplineComponent.GetLocationAtTime` (`self.Spline`) `_新建轨道_0` "World" false) false false))
      (:`Finished`
        (`KismetSystemLibrary.Delay` 1.0)
        (`self.Complete Event`)
        (`self.K2_DestroyActor`)))))

(fn `UserConstructionScript`)