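; BP_Door_Level_one is a level exit gate that shows the game end menu when the player passes through it.
; On actor overlap it checks for the "player" tag and that the ConditionalDataOnPassageThroughTheGate collection is empty.
; When both hold, it creates the GameEnd_Menu widget, adds it to the viewport and shows the mouse cursor.
; Nothing in these graphs fills or empties that collection.
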(event `self.ReceiveActorBeginOverlap`
  (params (OtherActor :type "Actor Object Reference"))
  (if (`self.ActorHasTag` OtherActor "player")
    (if (<= (`KismetArrayLibrary.Array_Length` (`self.Conditional Data On Passage Through The Gate`)) 0)
      (bind _returnvalue (`|CreateWidget` "/Game/CombatSystem/Menu/GameEnd_Menu.GameEnd_Menu_C"))
      (`UserWidget.AddToViewport` _returnvalue 0)
      (set `PlayerController.bShowMouseCursor` true (`GameplayStatics.GetPlayerController` 0)))))

(fn `UserConstructionScript`
  (`parent.UserConstructionScript`))