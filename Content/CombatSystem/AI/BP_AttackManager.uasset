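; BP_AttackManager is a combat AI manager that hands out attack permission to NPCs, aiming to limit simultaneous attackers.
; From BeginPlay, 请求攻击 counts attacking entries in NPCData, clears their AttackPermission and pools the rest.
; Below the maximum, it grants permission to random pool picks (repeats possible) for the free slots, then re-runs after a short Delay.
; At the maximum, the loop does not reschedule itself.
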(event `self.ReceiveBeginPlay`
  (`self.请求攻击`))

(event `请求攻击`
  (bind _output (`|GetArrayItem` (`self.可攻击NPC`) (`self.执行攻击 ID`)))
  (`KismetArrayLibrary.Array_Clear` (`self.可攻击NPC`))
  (set `self.正在攻击的人数` 0)
  (for _array_element (`self.NPC Data`)
    (if (`/Game/CombatSystem/AI/BP_AI_Character.Attacking` _array_element)
      (`/Engine/EditorBlueprintResources/StandardMacros.IncrementInt` (`self.正在攻击的人数`)
        (:`  `
          (set `/Game/CombatSystem/AI/BP_AI_Character.Attack Permission` false _array_element)))
      (else
        (`KismetArrayLibrary.Array_Add` (`self.可攻击NPC`) _array_element))))
  (if (< (`self.正在攻击的人数`) (`self.最大同时攻击的人数`))
    (set `self.还可以进行攻击的人数` (- (`self.最大同时攻击的人数`) (`self.正在攻击的人数`)))
    (for _ (range 1 (+ (`self.还可以进行攻击的人数`) 1))
      (set `self.执行攻击 ID` (`KismetMathLibrary.RandomIntegerInRange` 0 (- (`KismetArrayLibrary.Array_Length` (`self.可攻击NPC`)) 1)))
      (`/Engine/EditorBlueprintResources/StandardMacros.IsValid` _output
        (:`Is Valid`
          (set `/Game/CombatSystem/AI/BP_AI_Character.Attack Permission` true _output))))
    (`KismetSystemLibrary.Delay` 0.2)
    (`self.请求攻击`)))

(fn `UserConstructionScript`)