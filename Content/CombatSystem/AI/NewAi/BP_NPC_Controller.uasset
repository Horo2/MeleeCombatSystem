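; NPC AI controller that runs a behavior tree and switches its state between chasing, EQS standby, attacking and post-attack retreat.
; Data table rows become named looping timers that act as services, paused or resumed per state.
; A sphere-trace service finds Player-tagged pawns in standby or attack range, and another polls the character for attack permission.
; Their results, attack completion and behavior tree completion events drive state and walk speed changes.
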(event `初始化数据`
  ;[1 1 1] 初始化服务数据
  (bind _outrownames (`DataTableFunctionLibrary.GetDataTableRowNames` "/Game/CombatSystem/AI/NewAi/NPCServiceDataTable.NPCServiceDataTable"))
  (for _array_element _outrownames
    (bind _returnvalue (`|GetDataTableRow` "/Game/CombatSystem/AI/NewAi/NPCServiceDataTable.NPCServiceDataTable" _array_element)
      (:`then`
        (`KismetArrayLibrary.Array_Add` (`self.Service Sturct`) _returnvalue))))
  (for (_array_element_2 _array_index) (`self.Service Sturct`)
    (bind _servicename (break `/Game/CombatSystem/AI/NewAi/Service_Struct` _array_element_2))
    (bind _returnvalue_2 (`KismetSystemLibrary.K2_SetTimer` null _servicename 0.1 true))
    (`|VariableSetRef` (`|GetArrayItem` (`self.Service Sturct`) _array_index) (make `/Game/CombatSystem/AI/NewAi/Service_Struct` _servicename _returnvalue_2)))
  (`self.激活或关闭服务` false))

(event `self.ReceiveBeginPlay`
  (bind `_as角色` (cast `Character` (`self.K2_GetPawn`)))
  (set `self.BP NPC Character` `_as角色`)
  (`self.初始化数据`)
  (`self.RunBehaviorTree` "/Game/CombatSystem/AI/NewAi/BT_NPC_AI_BehaviourTree.BT_NPC_AI_BehaviourTree")
  (`self.设置NPC行为逻辑` "NewEnumerator5"))

(event `搜索结果处理`
  (params (SearchTpyeEnum :type "/Game/CombatSystem/AI/NewAi/SearchTpyeEnum Enum" :default "SearchTpyeEnum_MAX") (`Serch Results` :type Boolean))
  (bind _bp_npc_character (`self.BP NPC Character`))
  (if `Serch Results`
    (switch `/Game/CombatSystem/AI/NewAi/Enum_BehaviourTreeBehaviour` (`self.Behaviour Tree Behaviour`)
      (:`NewEnumerator5`
        (bind _returnvalue (`|GetDataTableRow` "/Game/CombatSystem/AI/NewAi/NPCServiceDataTable.NPCServiceDataTable" "搜索服务函数")
          (:`then`
            (`self.激活或关闭服务` false (break `/Game/CombatSystem/AI/NewAi/Service_Struct` _returnvalue))
            (`/Game/CombatSystem/AI/Component/NPC_BehavioralComponents.Activate Focus Fo Player` (`self.GetComponentByClass` (`self.BP NPC Character`) "/Game/CombatSystem/AI/Component/NPC_BehavioralComponents.NPC_BehavioralComponents_C"))
            (`self.设置NPC行为逻辑` "NewEnumerator6")
            (bind _returnvalue_2 (`|GetDataTableRow` "/Game/CombatSystem/AI/NewAi/NPCServiceDataTable.NPCServiceDataTable" "查询攻许可击服务函数")
              (:`then`
                (`self.激活或关闭服务` true (break `/Game/CombatSystem/AI/NewAi/Service_Struct` _returnvalue_2)))))))
      (:`NewEnumerator9`
        (`self.设置NPC行为逻辑` "NewEnumerator0")
        (bind _returnvalue_3 (`|GetDataTableRow` "/Game/CombatSystem/AI/NewAi/NPCServiceDataTable.NPCServiceDataTable" "搜索服务函数")
          (:`then`
            (`self.激活或关闭服务` false (break `/Game/CombatSystem/AI/NewAi/Service_Struct` _returnvalue_3))
            (message `/Game/CombatSystem/AI/NPCData/NPC_Interface.Attack` _bp_npc_character)
            (bind _asbp_ai_character (cast `/Game/CombatSystem/AI/BP_AI_Character` _bp_npc_character))
            (add `/Game/CombatSystem/AI/BP_AI_Character.Attack Completion Event` _asbp_ai_character (delegate `NPC Attack Completion`))))))))

(event `NPC Attack Completion`
  (`self.设置NPC行为逻辑` "NewEnumerator10"))

(event `行为树完成执行处理`
  (params (`Behaviour Tree Behaviour` :type "/Game/CombatSystem/AI/NewAi/Enum_BehaviourTreeBehaviour Enum" :default "NewEnumerator0"))
  (switch `/Game/CombatSystem/AI/NewAi/Enum_BehaviourTreeBehaviour` `Behaviour Tree Behaviour`
    (:`NewEnumerator6`
      (`self.设置NPC行为逻辑` "NewEnumerator7"))
    (:`NewEnumerator7`
      (bind _npc_data (message `/Game/CombatSystem/AI/NPCData/NPC_Interface.Get NPC Data` (`self.BP NPC Character`)))
      (set `CharacterMovementComponent.MaxWalkSpeed` (`.攻击待机移动速度_13_B2D036C4405F9CEAE480AE98E67603CF` (break `/Game/CombatSystem/AI/NPCData/NPCData_Struct` _npc_data)) (`Character.CharacterMovement` (`self.BP NPC Character`)))
      (`self.设置NPC行为逻辑` "NewEnumerator5"))
    (:`NewEnumerator10`
      (`self.设置NPC行为逻辑` "NewEnumerator11"))
    (:`NewEnumerator11`
      (bind _npc_data_2 (message `/Game/CombatSystem/AI/NPCData/NPC_Interface.Get NPC Data` (`self.BP NPC Character`)))
      (set `CharacterMovementComponent.MaxWalkSpeed` (`.攻击待机移动速度_13_B2D036C4405F9CEAE480AE98E67603CF` (break `/Game/CombatSystem/AI/NPCData/NPCData_Struct` _npc_data_2)) (`Character.CharacterMovement` (`self.BP NPC Character`)))
      (`self.设置NPC行为逻辑` "NewEnumerator5"))))

(event `设置NPC行为逻辑`
  (params (`Behaviour Tree Behaviour` :type "/Game/CombatSystem/AI/NewAi/Enum_BehaviourTreeBehaviour Enum" :default "NewEnumerator0"))
  (bind _output_get (set `self.Behaviour Tree Behaviour` `Behaviour Tree Behaviour`))
  (switch `/Game/CombatSystem/AI/NewAi/Enum_BehaviourTreeBehaviour` _output_get
    (:`NewEnumerator5`
      (bind _returnvalue (`|GetDataTableRow` "/Game/CombatSystem/AI/NewAi/NPCServiceDataTable.NPCServiceDataTable" "搜索服务函数")
        (:`then`
          (set `self.SearchTpyeEnum` "NewEnumerator0")
          (`self.激活或关闭服务` true (break `/Game/CombatSystem/AI/NewAi/Service_Struct` _returnvalue))
          (bind _npc_data (message `/Game/CombatSystem/AI/NPCData/NPC_Interface.Get NPC Data` (`self.BP NPC Character`)))
          (set `CharacterMovementComponent.MaxWalkSpeed` (`.追击移动速度_11_F1CC5DEB4628988A41C5BBB76B5C4140` (break `/Game/CombatSystem/AI/NPCData/NPCData_Struct` _npc_data)) (`Character.CharacterMovement` (`self.BP NPC Character`))))))
    (:`NewEnumerator8`
      (bind _returnvalue_2 (`|GetDataTableRow` "/Game/CombatSystem/AI/NewAi/NPCServiceDataTable.NPCServiceDataTable" "搜索服务函数")
        (:`then`
          (set `self.SearchTpyeEnum` "NewEnumerator1")
          (`self.激活或关闭服务` true (break `/Game/CombatSystem/AI/NewAi/Service_Struct` _returnvalue_2))
          (`self.设置NPC行为逻辑` "NewEnumerator9")
          (bind _npc_data_2 (message `/Game/CombatSystem/AI/NPCData/NPC_Interface.Get NPC Data` (`self.BP NPC Character`)))
          (set `CharacterMovementComponent.MaxWalkSpeed` (`.追击移动速度_11_F1CC5DEB4628988A41C5BBB76B5C4140` (break `/Game/CombatSystem/AI/NPCData/NPCData_Struct` _npc_data_2)) (`Character.CharacterMovement` (`self.BP NPC Character`))))))))

(fn `UserConstructionScript`)

(fn `搜索服务函数`
  (locals (`搜索结果` :type Boolean))
  (bind _returnvalue (`self.K2_GetActorLocation` (`self.BP NPC Character`)))
  (bind _npc_data (message `/Game/CombatSystem/AI/NPCData/NPC_Interface.Get NPC Data` (`self.BP NPC Character`)))
  (bind _outhits (`KismetSystemLibrary.SphereTraceMultiForObjects` _returnvalue _returnvalue (select `/Game/CombatSystem/AI/NewAi/SearchTpyeEnum` (`self.SearchTpyeEnum`) :`NewEnumerator0` (`.攻击待机范围_5_4D30ABBE4DE3FED8D312C3A3E788E327` (break `/Game/CombatSystem/AI/NPCData/NPCData_Struct` _npc_data)) :`NewEnumerator1` (break `/Game/CombatSystem/AI/NPCData/NPCData_Struct` _npc_data) :!type "Float (single-precision)") (`|MakeArray` "ObjectTypeQuery3" :!type "EObjectTypeQuery Enum") false (`|MakeArray` (`self.BP NPC Character`) :!type "Actor Object Reference")))
  (set `local.搜索结果` false)
  (for _array_element _outhits
    (if (`self.ActorHasTag` (`.HitActor` (`GameplayStatics.BreakHitResult` _array_element)) "Player")
      (set `local.搜索结果` true)))
  (`self.搜索结果处理` (`self.SearchTpyeEnum`) (`local.搜索结果`)))

(fn `查询攻许可击服务函数`
  (bind `_攻击许可` (message `/Game/CombatSystem/AI/NPCData/NPC_Interface.获取攻击许可` (`self.BP NPC Character`)))
  (set `self.攻击许可` `_攻击许可`)
  (if `_攻击许可`
    (`self.设置NPC行为逻辑` "NewEnumerator8")
    (bind _returnvalue (`|GetDataTableRow` "/Game/CombatSystem/AI/NewAi/NPCServiceDataTable.NPCServiceDataTable" "查询攻许可击服务函数")
      (:`then`
        (`self.激活或关闭服务` false (break `/Game/CombatSystem/AI/NewAi/Service_Struct` _returnvalue))))))

(fn `激活或关闭服务`
  (params (`激活` :type Boolean) (`服务名称` :type String))
  (locals (`Service Type Enum` :type "/Game/CombatSystem/AI/NewAi/Eunm_ServiceType Enum" :default "NewEnumerator0") (`服务名称 存` :type String))
  (set `local.服务名称 存` `服务名称`)
  (if (`KismetStringLibrary.IsEmpty` (`local.服务名称 存`))
    (for _array_element (`self.Service Sturct`)
      (if `激活`
        (`KismetSystemLibrary.K2_UnPauseTimerHandle` (`.Timer_5_60E765DE410DA1E91F6832AC5A26D033` (break `/Game/CombatSystem/AI/NewAi/Service_Struct` _array_element)))
        (else
          (`KismetSystemLibrary.K2_PauseTimerHandle` (`.Timer_5_60E765DE410DA1E91F6832AC5A26D033` (break `/Game/CombatSystem/AI/NewAi/Service_Struct` _array_element))))))
    (else
      (for _array_element_2 (`self.Service Sturct`)
        (if (== (break `/Game/CombatSystem/AI/NewAi/Service_Struct` _array_element_2) (`local.服务名称 存`))
          (if `激活`
            (`KismetSystemLibrary.K2_UnPauseTimerHandle` (`.Timer_5_60E765DE410DA1E91F6832AC5A26D033` (break `/Game/CombatSystem/AI/NewAi/Service_Struct` _array_element_2)))
            (else
              (`KismetSystemLibrary.K2_PauseTimerHandle` (`.Timer_5_60E765DE410DA1E91F6832AC5A26D033` (break `/Game/CombatSystem/AI/NewAi/Service_Struct` _array_element_2))))))))))