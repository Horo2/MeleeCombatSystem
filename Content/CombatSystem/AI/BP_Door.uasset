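; Combat door that can open only once its registered NPCs are all gone, then shuts behind the player.
; A looping timer prunes invalid NPCs, which can be added at runtime, and sets the open condition when none remain.
; An open request plays a timeline once; a player-tagged overlap on PassDoorBOX reverses it once.
; AnimationToDoor is an empty hook here; the construction script positions the button mesh and pass-through box.
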(event `self.ReceiveBeginPlay`
  (bind _returnvalue (`KismetSystemLibrary.K2_SetTimerDelegate` (delegate `开门判断条件`) 0.2 true))
  (set `self.开门条件定时器` _returnvalue))

(event `self.ReceiveTick`
  (params (DeltaSeconds :type "Float (single-precision)")))

(event `动态添加NPC`
  (params (`Spawn NPC` :type "Actor Object Reference (by ref)"))
  (`KismetArrayLibrary.Array_Add` (`self.Conditional Data On Passage Through The Gate`) `Spawn NPC`))

(event `开门判断条件`
  (for (_array_element _array_index) (`self.Conditional Data On Passage Through The Gate`)
    (`/Engine/EditorBlueprintResources/StandardMacros.IsValid` _array_element
      (:`Is Not Valid`
        (`KismetArrayLibrary.Array_Remove` (`self.Conditional Data On Passage Through The Gate`) _array_index))))
  (if (<= (`KismetArrayLibrary.Array_Length` (`self.Conditional Data On Passage Through The Gate`)) 0)
    (set `self.开门条件` true)
    (else
      (set `self.开门条件` false))))

(event `请求开门`
  (if (`self.开门条件`)
    (`/Engine/EditorBlueprintResources/StandardMacros.DoOnce` false
      (:`Completed`
        (`self.Open Door`)))))

(event `Open Door`
  (bind (_direction `_新建轨道_0`) (`Timeline|Open The Door Animation` :!via `PlayFromStart` :!label _label)
    (:`Update`
      (`self.Animation To Door` `_新建轨道_0`))))

(event `Close Door`
  (goto _label :!via `ReverseFromEnd`))

(event `Animation To Door`
  (params (Time :type "Float (double-precision)")))

(event `Complete The Door Animation`)

(event `self.Pass Door BOX.OnComponentBeginOverlap`
  (params (OverlappedComponent :type "PrimitiveComponent Object Reference") (OtherActor :type "Actor Object Reference") (OtherComp :type "PrimitiveComponent Object Reference") (OtherBodyIndex :type Integer) (bFromSweep :type Boolean) (SweepResult :type "HitResult Structure (by ref)"))
  (`/Engine/EditorBlueprintResources/StandardMacros.IsValid` OtherActor
    (:`Is Valid`
      (if (`self.ActorHasTag` OtherActor "Player")
        (`/Engine/EditorBlueprintResources/StandardMacros.DoOnce` false
          (:`Completed`
            (`self.Close Door`)))))))

(event `self.Box.OnComponentBeginOverlap`
  (params (OverlappedComponent :type "PrimitiveComponent Object Reference") (OtherActor :type "Actor Object Reference") (OtherComp :type "PrimitiveComponent Object Reference") (OtherBodyIndex :type Integer) (bFromSweep :type Boolean) (SweepResult :type "HitResult Structure (by ref)"))
  (`/Engine/EditorBlueprintResources/StandardMacros.IsValid` OtherActor
    (:`Is Valid`
      (if (`self.ActorHasTag` OtherActor "Player")
        _))))

(fn `UserConstructionScript`
  (`SceneComponent.K2_SetRelativeTransform` (`self.SM_Prop_Buttons_07`) (`self.Key Transform`) false false)
  (`SceneComponent.K2_SetRelativeTransform` (`self.Pass Door BOX`) (`self.Pass Door Collision BOX Transform`) false false))