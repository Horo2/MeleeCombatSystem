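; BP_AI_Character is an AI character in the combat system that can turn to face the player.
; On BeginPlay it finds BP_AttackManager and adds itself to that manager's NPCData list.
; PlayerRotationAnimation uses a timeline to lerp yaw toward the player's location, calling itself again on finish until StopRotationAnimation stops the timeline.
; GetNPCData exposes the character's own NPCData.
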(event `self.ReceiveBeginPlay`
  (bind _returnvalue (`GameplayStatics.GetActorOfClass` "/Game/CombatSystem/AI/BP_AttackManager.BP_AttackManager_C"))
  (`KismetArrayLibrary.Array_Add` (`/Game/CombatSystem/AI/BP_AttackManager.NPC Data` _returnvalue) self))

(event `Player Rotation Animation`
  (bind (_returnvalue_roll _returnvalue_pitch _returnvalue_yaw) (`KismetMathLibrary.BreakRotator` (`self.K2_GetActorRotation`)))
  (bind (_returnvalue_roll_2 _returnvalue_pitch_2 _returnvalue_yaw_2) (`KismetMathLibrary.BreakRotator` (`KismetMathLibrary.FindLookAtRotation` (`self.K2_GetActorLocation`) (`self.K2_GetActorLocation` (`GameplayStatics.GetPlayerCharacter` 0)))))
  (set `self.Return Value Z (Yaw)` _returnvalue_yaw)
  (bind (_direction `_新建轨道_0`) (`Timeline|时间轴` :!label _label)
    (:`Update`
      (`self.K2_SetActorRotation` (`KismetMathLibrary.MakeRotator` 0.0 0.0 (`KismetMathLibrary.Lerp` (`self.Return Value Z (Yaw)`) _returnvalue_yaw_2 `_新建轨道_0`))))
    (:`Finished`
      (`self.Player Rotation Animation`))))

(event `Stop Rotation Animation`
  (goto _label :!via `Stop`))

(fn `Get NPC Data`
  (returns (`NPC Data` :type "/Game/CombatSystem/AI/NPCData_Struct Structure"))
  (return (`self.NPC Data`)))

(fn `UserConstructionScript`)