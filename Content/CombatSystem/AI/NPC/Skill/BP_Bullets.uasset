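; BP_Bullets is a projectile actor for NPC skills that damages the player on overlap.
; BeginPlay applies its mesh and starts its Niagara or particle effect.
; Tick moves it along its Arrow's forward vector without sweeping or delta-time scaling.
; Sphere overlap calls TakeDamage with interruption on a Player-tagged hit actor's BP_StatsComponent, leaving the bullet alive; other overlaps destroy it.
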(event `self.ReceiveBeginPlay`
  (`StaticMeshComponent.SetStaticMesh` (`self.Remote_Bullet`) (`self.Bullets Stataic Mehs`))
  (`NiagaraComponent.SetAsset` (`self.Remote_NormalAttack_Fire`) (`self.In Asset`) true)
  (`ActorComponent.SetActive` (`self.Remote_NormalAttack_Fire`) true true))

(event `self.ReceiveTick`
  (params (DeltaSeconds :type "Float (single-precision)"))
  (`self.K2_AddActorWorldOffset` (* (`SceneComponent.GetForwardVector` (`self.Arrow`)) (`self.Bullets Speed`))))

(event `self.Sphere.OnComponentBeginOverlap`
  (params (OverlappedComponent :type "PrimitiveComponent Object Reference") (OtherActor :type "Actor Object Reference") (OtherComp :type "PrimitiveComponent Object Reference") (OtherBodyIndex :type Integer) (bFromSweep :type Boolean) (SweepResult :type "HitResult Structure (by ref)"))
  (bind (_bblockinghit _binitialoverlap _time _distance _location _impactpoint _normal _impactnormal _physmat _hitactor) (`GameplayStatics.BreakHitResult` SweepResult))
  (`/Engine/EditorBlueprintResources/StandardMacros.IsValid` (`self.GetComponentByClass` OtherActor "/Game/CombatSystem/Blueprints/Components/BP_StatsComponent.BP_StatsComponent_C")
    (:`Is Valid`
      (if (`self.ActorHasTag` _hitactor "Player")
        (`/Game/CombatSystem/Blueprints/Components/BP_StatsComponent.TakeDamage` (`self.GetComponentByClass` _hitactor "/Game/CombatSystem/Blueprints/Components/BP_StatsComponent.BP_StatsComponent_C") (`self.In Damage`) self true)
        (else
          (`self.K2_DestroyActor`))))
    (:`Is Not Valid`
      (`self.K2_DestroyActor`))))

(fn `UserConstructionScript`)