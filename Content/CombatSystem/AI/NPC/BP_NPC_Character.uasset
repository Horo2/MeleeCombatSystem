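; NPC combat character that turns toward the player and automatically jumps up ledges along its AI path.
; A polling loop pathfinds to the move destination and, for short, steep climbs, spawns BP_JumpingCurve to drive the jump, resuming on completion.
; ActivateEnemyService toggles a repeating Timeline yaw turn toward the player against controller-driven yaw.
; Attack and PointDamage are empty; hit-reaction, knock-up and damage logic remains only as disconnected nodes.
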(event `self.ReceiveBeginPlay`
  (`self.Jumping`))

(event `Attack`)

(event `Activate Enemy Service`
  (params (`Activate?` :type Boolean))
  (if `Activate?`
    (set `self.bUseControllerRotationYaw` false)
    (`self.Playe Rotation Animation`)
    (else
      (set `self.bUseControllerRotationYaw` true)
      (`self.Stop Rotation Animation`))))

(event `Playe Rotation Animation`
  (bind (_returnvalue_roll _returnvalue_pitch _returnvalue_yaw) (`KismetMathLibrary.BreakRotator` (`self.K2_GetActorRotation`)))
  (bind _returnvalue (`GameplayStatics.GetPlayerCharacter` 0))
  (bind (_returnvalue_roll_2 _returnvalue_pitch_2 _returnvalue_yaw_2) (`KismetMathLibrary.BreakRotator` (`KismetMathLibrary.FindLookAtRotation` (`self.K2_GetActorLocation`) (`self.K2_GetActorLocation` _returnvalue))))
  ;[1 1 1] 转身动画
  (set `self.Iteslf Rotation` _returnvalue_yaw)
  (bind (_direction `_新建轨道_0`) (`Timeline|时间轴` :!label _label)
    (:`Update`
      (`/Engine/EditorBlueprintResources/StandardMacros.IsValid` _returnvalue
        (:`Is Valid`
          (`self.K2_SetActorRotation` self (`KismetMathLibrary.MakeRotator` 0.0 0.0 (`KismetMathLibrary.Lerp` (`self.Iteslf Rotation`) _returnvalue_yaw_2 `_新建轨道_0`)) false))))
    (:`Finished`
      (`self.Playe Rotation Animation`))))

(event `Stop Rotation Animation`
  ;[1 1 1] 转身动画
  (goto _label :!via `Stop`))

(event `Jumping`
  (bind (_returnvalue_location _returnvalue_rotation) (`KismetMathLibrary.BreakTransform` (`self.GetTransform`)))
  (bind _path_points (`self.Path Points`))
  (bind (_output_x _output_y _output_z) (`KismetMathLibrary.BreakVector` (`|GetArrayItem` (`self.Path Points`))))
  (bind (_output_x_2 _output_y_2 _output_z_2) (`KismetMathLibrary.BreakVector` (`|GetArrayItem` (`self.Path Points`) 2)))
  ;[1 1 1] 跳跃动画
  (`KismetSystemLibrary.Delay` 0.2)
  (bind _returnvalue (`NavigationSystemV1.FindPathToLocationSynchronously` (`self.K2_GetActorLocation`) (`AIController.GetImmediateMoveDestination` (`AIBlueprintHelperLibrary.GetAIController` self)) self null))
  (`/Engine/EditorBlueprintResources/StandardMacros.IsValid` _returnvalue
    (:`Is Valid`
      (bind _output_get (set `self.Path Points` (`NavigationPath.PathPoints` _returnvalue)))
      (bind _returnvalue_2 (`KismetArrayLibrary.Array_Length` _output_get))
      (if (== _returnvalue_2 2)
        (`KismetArrayLibrary.Array_Add` (`self.Path Points`) (* (+ (`|GetArrayItem` _path_points) (`|GetArrayItem` _path_points 1)) (`KismetStringLibrary.Conv_StringToDouble` "2")))
        (`KismetArrayLibrary.Array_Swap` (`self.Path Points`) 1 2)
        (if (and (> (- _output_z_2 _output_z) 80.0) (< (`KismetMathLibrary.Vector_Distance` (`|GetArrayItem` (`self.Path Points`)) (`|GetArrayItem` (`self.Path Points`) 2)) 400.0)) :!label _label_2
          (`KismetSystemLibrary.Delay` 0.3)
          (bind _returnvalue_3 (`|SpawnActorFromClass` "/Game/CombatSystem/AI/BP_JumpingCurve.BP_JumpingCurve_C" (`KismetMathLibrary.MakeTransform` _returnvalue_location _returnvalue_rotation) "AlwaysSpawn" "MultiplyWithRoot" null (`self.Path Points`) self 1.0 null))
          (`self.Jump`)
          (add `/Game/CombatSystem/AI/BP_JumpingCurve.Complete Event` _returnvalue_3 (delegate `Custom Jumping Event`))
          (else
            (`self.Jumping`)))
        (elif (> _returnvalue_2 2)
          (goto _label_2)
          (else
            (`self.Jumping`)))))
    (:`Is Not Valid`
      (`self.Jumping`))))

(event `Custom Jumping Event`
  ;[1 1 1] 跳跃动画
  (`self.Jumping`))

(event `self.ReceivePointDamage`
  (params (Damage :type "Float (single-precision)") (DamageType :type "DamageType Object Reference") (HitLocation :type "Vector Structure") (HitNormal :type "Vector Structure") (HitComponent :type "PrimitiveComponent Object Reference") (BoneName :type Name) (ShotFromDirection :type "Vector Structure") (InstigatedBy :type "Controller Object Reference") (DamageCauser :type "Actor Object Reference") (HitInfo :type "HitResult Structure (by ref)"))
  ;[1 0 0] Damage
)

(fn `CanRecieveDamage`
  (returns (ReturnValue :type Boolean))
  (return (`self.Recieve Damage`)))

(fn `GetDesiredRotation`
  (returns (ReturnValue :type "Rotator Structure"))
  (return))

(fn `UserConstructionScript`)