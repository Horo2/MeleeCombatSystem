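; Test NPC Blueprint that continuously traces a navigation path from itself to the player character and lays it out on a Spline component.
; A self-calling Jumping event, started on BeginPlay, waits 0.2 seconds, then runs a synchronous navmesh path query.
; Each valid result rebuilds the spline from the path points in world space, deferring the spline update until all points are added.
; Nothing here moves the actor along the path.
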(event `self.ReceiveBeginPlay`
  (`self.Jumping`))

(event `Jumping`
  (`KismetSystemLibrary.Delay` 0.2)
  (bind _returnvalue (`NavigationSystemV1.FindPathToLocationSynchronously` (`self.K2_GetActorLocation`) (`self.K2_GetActorLocation` (`GameplayStatics.GetPlayerCharacter` 0)) self null))
  (`/Engine/EditorBlueprintResources/StandardMacros.IsValid` _returnvalue
    (:`Is Valid`
      (`SplineComponent.ClearSplinePoints` (`self.Spline`) true)
      (for _array_element (`NavigationPath.PathPoints` _returnvalue)
        (`SplineComponent.AddSplinePoint` (`self.Spline`) _array_element "World" false))
      (`SplineComponent.UpdateSpline` (`self.Spline`))
      (`self.Jumping`))
    (:`Is Not Valid`
      (`self.Jumping`))))

(fn `UserConstructionScript`)